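; BP_MesaEquipamiento is an interactable equipment table that hands the player their gear once.
; On interact it unlocks four tools in AC_Inventario, adds two ammo types, equips the first tool and installs the sensor through AC_Detector.
; It then hides the items, marks itself used, which blanks the prompt, and sends a game-instance notification.
; Scanning highlights the mesh through custom depth stencil with a timer.
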(event `self.ReceiveBeginPlay`)

(event `/Game/EstacionNueve/Core/BPI_Interactuable.E_OnInteract`
  (params (InstigatorActor :type "Actor Object Reference"))
  (bind _asac_inventario (cast `/Game/EstacionNueve/Componentes/AC_Inventario` (`self.GetComponentByClass` InstigatorActor "/Game/EstacionNueve/Componentes/AC_Inventario.AC_Inventario_C")))
  (bind _asac_detector (cast `/Game/EstacionNueve/Componentes/AC_Detector` (`self.GetComponentByClass` InstigatorActor "/Game/EstacionNueve/Componentes/AC_Detector.AC_Detector_C")))
  (if (not (`self.bUsada`))
    (`/Game/EstacionNueve/Componentes/AC_Inventario.DesbloquearHerramienta` _asac_inventario "NewEnumerator1")
    (`/Game/EstacionNueve/Componentes/AC_Inventario.DesbloquearHerramienta` _asac_inventario "NewEnumerator2")
    (`/Game/EstacionNueve/Componentes/AC_Inventario.DesbloquearHerramienta` _asac_inventario "NewEnumerator3")
    (`/Game/EstacionNueve/Componentes/AC_Inventario.DesbloquearHerramienta` _asac_inventario "NewEnumerator4")
    (`/Game/EstacionNueve/Componentes/AC_Inventario.Agregar` _asac_inventario "Balas44" 18)
    (`/Game/EstacionNueve/Componentes/AC_Inventario.Agregar` _asac_inventario "Cartuchos" 8)
    (`/Game/EstacionNueve/Componentes/AC_Inventario.EquiparHerramienta` _asac_inventario "NewEnumerator1")
    (`/Game/EstacionNueve/Componentes/AC_Detector.InstalarSensor` _asac_detector)
    (`SceneComponent.SetVisibility` (`self.Objetos`) false false)
    (set `self.bUsada` true)
    (bind _asbp_gi_estacion_nueve (cast `/Game/EstacionNueve/Core/BP_GI_EstacionNueve` (`GameplayStatics.GetGameInstance`)))
    (`/Game/EstacionNueve/Core/BP_GI_EstacionNueve.Notificar` _asbp_gi_estacion_nueve "Equipo: Rayo [1], Pico [2], Revólver [3], Escopeta [4], Sensor [Q]")))

(event `self.ReceiveActorBeginOverlap`
  (params (OtherActor :type "Actor Object Reference")))

(event `self.ReceiveTick`
  (params (DeltaSeconds :type "Float (single-precision)")))

(event `/Game/EstacionNueve/Core/BPI_Interactuable.E_OnScanned`
  (params (SensorLevel :type Integer))
  (bind _malla (`self.Malla`))
  (`PrimitiveComponent.SetRenderCustomDepth` _malla true)
  (`PrimitiveComponent.SetCustomDepthStencilValue` _malla (`self.StencilEscaneo`))
  (`KismetSystemLibrary.K2_SetTimerDelegate` (`|CreateDelegate` :!event `FinResaltado`) 4.0))

(event `FinResaltado`
  (`PrimitiveComponent.SetRenderCustomDepth` (`self.Malla`) false))

(event `/Game/EstacionNueve/Core/BPI_Interactuable.E_Fire`)

(event `/Game/EstacionNueve/Core/BPI_Interactuable.E_Reload`)

(event `/Game/EstacionNueve/Core/BPI_Interactuable.E_Hit`)

(fn `GetInteractionPrompt`
  (returns (Prompt :type Text))
  (if (`self.bUsada`)
    (return (`KismetTextLibrary.Conv_StringToText` ""))
    (else
      (return (`KismetTextLibrary.Conv_StringToText` "Tomar equipo")))))

(fn `UserConstructionScript`)