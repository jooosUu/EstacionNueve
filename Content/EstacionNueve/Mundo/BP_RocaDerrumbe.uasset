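; BP_RocaDerrumbe is a cave-in rock that the Compressor Ray can compress and relaunch as a crushing physics projectile.
; Compression disables its collision; decompression restores collision, enables physics and applies a mass-independent launch impulse.
; A sufficiently fast hit applies crush damage and reports noise to the GameInstance once, until the next decompression rearms it.
; Scanning highlights the mesh through custom depth stencil until a short timer clears it.
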(event `self.ReceiveBeginPlay`)

(event `self.E_OnCompressed`
  (`self.SetActorEnableCollision` false)
  (`PrimitiveComponent.SetCollisionEnabled` (`self.Malla`) "NoCollision"))

(event `self.E_OnDecompressed`
  (params (LaunchImpulse :type "Vector Structure"))
  (bind _malla (`self.Malla`))
  (`PrimitiveComponent.SetCollisionEnabled` _malla "QueryAndPhysics")
  (`PrimitiveComponent.SetSimulatePhysics` _malla true)
  (`PrimitiveComponent.AddImpulse` _malla LaunchImpulse "None" true)
  (set `self.bGolpeAplicado` false))

(event `self.Malla.OnComponentHit`
  (params (HitComponent :type "PrimitiveComponent Object Reference") (OtherActor :type "Actor Object Reference") (OtherComp :type "PrimitiveComponent Object Reference") (NormalImpulse :type "Vector Structure") (Hit :type "HitResult Structure (by ref)"))
  (bind _returnvalue (`PrimitiveComponent.GetPhysicsLinearVelocity` (`self.Malla`) "None"))
  (if (and (not (`self.bGolpeAplicado`)) (> (`KismetMathLibrary.VSize` _returnvalue) (`self.VelocidadImpactoMinima`)))
    (set `self.bGolpeAplicado` true)
    (`GameplayStatics.ApplyDamage` OtherActor (`self.DanoAplastamiento`) null self "/Game/EstacionNueve/Core/DT_Aplastamiento.DT_Aplastamiento_C")
    (bind _asbp_gi_estacion_nueve (cast `/Game/EstacionNueve/Core/BP_GI_EstacionNueve` (`GameplayStatics.GetGameInstance` self)))
    (`/Game/EstacionNueve/Core/BP_GI_EstacionNueve.ReportNoise` _asbp_gi_estacion_nueve (`self.K2_GetActorLocation` self) (`self.RuidoImpacto`) "NewEnumerator4" self)))

(event `self.E_OnScanned`
  (params (SensorLevel :type Integer))
  (bind _malla (`self.Malla`))
  (`PrimitiveComponent.SetRenderCustomDepth` _malla true)
  (`PrimitiveComponent.SetCustomDepthStencilValue` _malla (`self.StencilEscaneo`))
  (`KismetSystemLibrary.K2_SetTimer` null "FinResaltado" 4.0))

(event `self.ReceiveActorBeginOverlap`
  (params (OtherActor :type "Actor Object Reference")))

(event `self.ReceiveTick`
  (params (DeltaSeconds :type "Float (single-precision)")))

(fn `FinResaltado`
  (`PrimitiveComponent.SetRenderCustomDepth` (`self.Malla`) false))

(fn `GetInteractionPrompt`
  (returns (Prompt :type Text))
  (return (`KismetTextLibrary.Conv_StringToText` "Roca de derrumbe (usa el Rayo Compresor)")))

(fn `UserConstructionScript`)