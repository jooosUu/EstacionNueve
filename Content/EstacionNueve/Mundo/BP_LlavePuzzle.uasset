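; BP_LlavePuzzle is an interactable puzzle key pickup in EstacionNueve.
; On interact, it adds its ItemID and Cantidad to the instigator's AC_Inventario component, doing nothing if there is none.
; It then advances the objective to taking the key to the back door and shows a notification through BP_GI_EstacionNueve, then destroys itself.
; GetInteractionPrompt builds the "Recoger" prompt from quantity and item ID.
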(event `self.E_OnInteract`
  (params (InstigatorActor :type "Actor Object Reference"))
  (bind _asac_inventario (cast `/Game/EstacionNueve/Componentes/AC_Inventario` (`self.GetComponentByClass` InstigatorActor "/Game/EstacionNueve/Componentes/AC_Inventario.AC_Inventario_C")))
  (`/Game/EstacionNueve/Componentes/AC_Inventario.Agregar` _asac_inventario (`self.ItemID`) (`self.Cantidad`))
  (bind _asbp_gi_estacion_nueve (cast `/Game/EstacionNueve/Core/BP_GI_EstacionNueve` (`GameplayStatics.GetGameInstance`))
    (:`then`
      (`/Game/EstacionNueve/Core/BP_GI_EstacionNueve.SetObjetivo` _asbp_gi_estacion_nueve "Lleva la llave a la puerta del fondo (E)" 2)
      (bind _asbp_gi_estacion_nueve_2 (cast `/Game/EstacionNueve/Core/BP_GI_EstacionNueve` (`GameplayStatics.GetGameInstance`)))
      (`/Game/EstacionNueve/Core/BP_GI_EstacionNueve.Notificar` _asbp_gi_estacion_nueve_2 "Recogiste la llave"))
    (:`CastFailed`
      _))
  (`self.K2_DestroyActor`))

(fn `GetInteractionPrompt`
  (returns (Prompt :type Text))
  (return (`KismetTextLibrary.Conv_StringToText` (`KismetStringLibrary.Concat_StrStr` (`KismetStringLibrary.Concat_StrStr` (`KismetStringLibrary.Concat_StrStr` (`KismetStringLibrary.Concat_StrStr` "Recoger" " ") (`KismetStringLibrary.Conv_IntToString` (`self.Cantidad`))) " ") (`KismetStringLibrary.Conv_NameToString` (`self.ItemID`))))))

(fn `UserConstructionScript`)