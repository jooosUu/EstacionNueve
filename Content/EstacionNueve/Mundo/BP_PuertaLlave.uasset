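; BP_PuertaLlave is an interactable locked door that consumes "Llave" items to unlock permanently and advance the objective.
; A timeline swings the hinge open, while closing only clears Abierta without animating.
; The interaction prompt checks and mentions diamonds instead of the key, though both use CosteDiamantes as quantity.
; Scanning highlights Compuerta through custom depth stencil until a timer clears it.
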(event `self.ReceiveBeginPlay`)

(event `self.ReceiveActorBeginOverlap`
  (params (OtherActor :type "Actor Object Reference")))

(event `self.E_OnInteract`
  (params (InstigatorActor :type "Actor Object Reference"))
  (bind _costediamantes (`self.CosteDiamantes`))
  (if (`self.bAbierta`)
    (set `self.bAbierta` false)
    (elif (`self.bDesbloqueada`)
      (set `self.bAbierta` true :!label _label)
      (bind (_direction _angulo) (`Timeline|Timeline_Apertura` :!via `PlayFromStart`)
        (:`Update`
          (`SceneComponent.K2_SetRelativeRotation` (`self.Bisagra`) (`KismetMathLibrary.MakeRotator` 0.0 0.0 _angulo) false false)))
      (else
        (bind _asac_inventario (cast `/Game/EstacionNueve/Componentes/AC_Inventario` (`self.GetComponentByClass` InstigatorActor "/Game/EstacionNueve/Componentes/AC_Inventario.AC_Inventario_C")))
        (if (`/Game/EstacionNueve/Componentes/AC_Inventario.Tiene` _asac_inventario "Llave" _costediamantes)
          (`/Game/EstacionNueve/Componentes/AC_Inventario.Quitar` _asac_inventario "Llave" _costediamantes)
          (bind _asbp_gi_estacion_nueve (cast `/Game/EstacionNueve/Core/BP_GI_EstacionNueve` (`GameplayStatics.GetGameInstance`))
            (:`then`
              (`/Game/EstacionNueve/Core/BP_GI_EstacionNueve.SetObjetivo` _asbp_gi_estacion_nueve "Cruza la puerta y llega a la zona de refugio" 3))
            (:`CastFailed`
              _))
          (set `self.bDesbloqueada` true)
          (goto _label)
          (else
            (bind _asbp_gi_estacion_nueve_2 (cast `/Game/EstacionNueve/Core/BP_GI_EstacionNueve` (`GameplayStatics.GetGameInstance`)))
            (`/Game/EstacionNueve/Core/BP_GI_EstacionNueve.Notificar` _asbp_gi_estacion_nueve_2 "Necesitas la llave")))))))

(event `self.ReceiveTick`
  (params (DeltaSeconds :type "Float (single-precision)")))

(event `self.E_OnScanned`
  (params (SensorLevel :type Integer))
  (bind _compuerta (`self.Compuerta`))
  (`PrimitiveComponent.SetRenderCustomDepth` _compuerta true)
  (`PrimitiveComponent.SetCustomDepthStencilValue` _compuerta (`self.StencilEscaneo`))
  (`KismetSystemLibrary.K2_SetTimer` self "FinResaltado" 4.0))

(event `self.E_OnCompressed`)

(event `self.E_OnDecompressed`
  (params (LaunchImpulse :type "Vector Structure")))

(event `self.E_Fire`)

(event `self.E_Reload`)

(event `self.E_Hit`)

(fn `FinResaltado`
  (bind _compuerta (`self.Compuerta`))
  (`PrimitiveComponent.SetRenderCustomDepth` _compuerta false)
  (`PrimitiveComponent.SetCustomDepthStencilValue` _compuerta 0))

(fn `GetInteractionPrompt`
  (returns (Prompt :type Text))
  (if (`self.bAbierta`)
    (return "")
    (else
      (bind _asac_inventario (cast `/Game/EstacionNueve/Componentes/AC_Inventario` (`self.GetComponentByClass` (`GameplayStatics.GetPlayerPawn` self) null))
        (:`then`
          (if (`/Game/EstacionNueve/Componentes/AC_Inventario.Tiene` _asac_inventario "Diamante" (`self.CosteDiamantes`))
            (return "Pagar 3 Diamantes")
            (else
              (return (`|FormatText` "Necesitas 3 Diamantes (tienes {Tienes})" (`/Game/EstacionNueve/Componentes/AC_Inventario.GetCantidad` _asac_inventario "Diamante"))))))
        (:`CastFailed`
          (return ""))))))

(fn `UserConstructionScript`)