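; BP_ZonaRuidoAmbiental is a zone actor that sets the ambient noise level while the player is inside it.
; When the player pawn begins overlapping, it writes its NivelRuidoDb value to BP_GI_EstacionNueve through SetRuidoAmbiental.
; End overlap resets that value to zero without tracking other zones, so leaving one of several overlapping zones clears the noise level.
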(event `self.ReceiveActorBeginOverlap`
  (params (OtherActor :type "Actor Object Reference"))
  (if (== OtherActor (`GameplayStatics.GetPlayerPawn` 0))
    (bind _asbp_gi_estacion_nueve (cast `/Game/EstacionNueve/Core/BP_GI_EstacionNueve` (`GameplayStatics.GetGameInstance`)))
    (`/Engine/EditorBlueprintResources/StandardMacros.IsValid` _asbp_gi_estacion_nueve
      (:`Is Valid`
        (`/Game/EstacionNueve/Core/BP_GI_EstacionNueve.SetRuidoAmbiental` _asbp_gi_estacion_nueve (`self.NivelRuidoDb`))))))

(event `self.ReceiveActorEndOverlap`
  (params (OtherActor :type "Actor Object Reference"))
  (if (== OtherActor (`GameplayStatics.GetPlayerPawn` 0))
    (bind _asbp_gi_estacion_nueve (cast `/Game/EstacionNueve/Core/BP_GI_EstacionNueve` (`GameplayStatics.GetGameInstance`)))
    (`/Engine/EditorBlueprintResources/StandardMacros.IsValid` _asbp_gi_estacion_nueve
      (:`Is Valid`
        (`/Game/EstacionNueve/Core/BP_GI_EstacionNueve.SetRuidoAmbiental` _asbp_gi_estacion_nueve 0.0)))))

(fn `UserConstructionScript`)