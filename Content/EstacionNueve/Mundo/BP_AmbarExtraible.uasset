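; BP_AmbarExtraible is an extractable amber capsule in EstacionNueve, whose interaction prompt points to the Compressor Ray.
; Scans at sufficient sensor level briefly highlight its mesh through custom depth, with a stencil value per level.
; Compression disables collision; decompression restores it, enables physics and launches the mesh with an impulse.
; Mesh hits report noise to the game instance, while interact, fire, reload and hit events are empty.
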(event `self.ReceiveBeginPlay`)

(event `/Game/EstacionNueve/Core/BPI_Interactuable.E_OnScanned`
  (params (SensorLevel :type Integer))
  (bind _malla (`self.Malla`))
  (bind _malla_2 (`self.Malla`))
  (if (>= SensorLevel 3)
    (`PrimitiveComponent.SetCustomDepthStencilValue` _malla (`self.StencilNivel3`))
    (`PrimitiveComponent.SetRenderCustomDepth` _malla true)
    (`KismetSystemLibrary.K2_SetTimerDelegate` (`|CreateDelegate` :!event `FinResaltado`) 4.0)
    (elif (>= SensorLevel 2)
      (`PrimitiveComponent.SetCustomDepthStencilValue` _malla_2 (`self.StencilNivel2`))
      (`PrimitiveComponent.SetRenderCustomDepth` _malla_2 true)
      (`KismetSystemLibrary.K2_SetTimerDelegate` (`|CreateDelegate` :!event `FinResaltado`) 4.0))))

(event `self.ReceiveActorBeginOverlap`
  (params (OtherActor :type "Actor Object Reference")))

(event `self.ReceiveTick`
  (params (DeltaSeconds :type "Float (single-precision)")))

(event `FinResaltado`
  (`PrimitiveComponent.SetRenderCustomDepth` (`self.Malla`) false))

(event `self.Malla.OnComponentHit`
  (params (HitComponent :type "PrimitiveComponent Object Reference") (OtherActor :type "Actor Object Reference") (OtherComp :type "PrimitiveComponent Object Reference") (NormalImpulse :type "Vector Structure") (Hit :type "HitResult Structure (by ref)"))
  (bind _asbp_gi_estacion_nueve (cast `/Game/EstacionNueve/Core/BP_GI_EstacionNueve` (`GameplayStatics.GetGameInstance` self)))
  (`/Game/EstacionNueve/Core/BP_GI_EstacionNueve.ReportNoise` _asbp_gi_estacion_nueve (`self.K2_GetActorLocation`) (`self.RuidoChoque`) "NewEnumerator4" self))

(event `/Game/EstacionNueve/Core/BPI_Interactuable.E_OnCompressed`
  (`self.SetActorEnableCollision` false)
  (`PrimitiveComponent.SetCollisionEnabled` (`self.Malla`) "NoCollision"))

(event `/Game/EstacionNueve/Core/BPI_Interactuable.E_OnDecompressed`
  (params (LaunchImpulse :type "Vector Structure"))
  (bind _malla (`self.Malla`))
  (`PrimitiveComponent.SetCollisionEnabled` _malla "QueryAndPhysics")
  (`PrimitiveComponent.SetSimulatePhysics` _malla true)
  (`PrimitiveComponent.AddImpulse` _malla LaunchImpulse "None" true))

(event `/Game/EstacionNueve/Core/BPI_Interactuable.E_OnInteract`
  (params (InstigatorActor :type "Actor Object Reference")))

(event `/Game/EstacionNueve/Core/BPI_Interactuable.E_Fire`)

(event `/Game/EstacionNueve/Core/BPI_Interactuable.E_Reload`)

(event `/Game/EstacionNueve/Core/BPI_Interactuable.E_Hit`)

(fn `GetInteractionPrompt`
  (returns (Prompt :type Text))
  (return (`KismetTextLibrary.Conv_StringToText` "Cápsula de Ámbar (usa el Rayo Compresor)")))

(fn `UserConstructionScript`)