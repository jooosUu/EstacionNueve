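; BP_ZonaRefugio is a shelter zone that marks the player as being in refuge while inside it.
; Overlap events on its Caja component filter for actors tagged "Jugador", then add the "EnRefugio" tag on entry and remove it on exit.
; The tag is the only state it sets, so any effect of sheltering is handled outside this Blueprint.
; Interaction and other stub events are disabled, and its interaction prompt is empty.
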(event `self.Caja.OnComponentBeginOverlap`
  (params (OverlappedComponent :type "PrimitiveComponent Object Reference") (OtherActor :type "Actor Object Reference") (OtherComp :type "PrimitiveComponent Object Reference") (OtherBodyIndex :type Integer) (bFromSweep :type Boolean) (SweepResult :type "HitResult Structure (by ref)"))
  (bind _temptags (`self.TempTags`))
  (if (`self.ActorHasTag` OtherActor "Jugador")
    (set `self.TempTags` (`Actor.Tags` OtherActor))
    (`KismetArrayLibrary.Array_Add` _temptags "EnRefugio")
    (set `Actor.Tags` _temptags OtherActor)))

(event `self.Caja.OnComponentEndOverlap`
  (params (OverlappedComponent :type "PrimitiveComponent Object Reference") (OtherActor :type "Actor Object Reference") (OtherComp :type "PrimitiveComponent Object Reference") (OtherBodyIndex :type Integer))
  (bind _temptags (`self.TempTags`))
  (if (`self.ActorHasTag` OtherActor "Jugador")
    (set `self.TempTags` (`Actor.Tags` OtherActor))
    (`KismetArrayLibrary.Array_RemoveItem` _temptags "EnRefugio")
    (set `Actor.Tags` _temptags OtherActor)))

(fn `GetInteractionPrompt`
  (returns (Prompt :type Text))
  (return ""))

(fn `UserConstructionScript`)