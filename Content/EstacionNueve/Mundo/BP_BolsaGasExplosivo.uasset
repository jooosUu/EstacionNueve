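; BP_BolsaGasExplosivo is an explosive gas pocket that detonates when damaged or when it registers a hit while its mesh moves faster than an impact threshold.
; Being scanned makes its membrane visible and briefly highlights the mesh through custom depth stencil, cleared by a timer.
; A one-shot explosion applies radial damage, reports noise to the game instance, then destroys the actor.
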(event `self.ReceiveBeginPlay`)

(event `/Game/EstacionNueve/Core/BPI_Interactuable.E_OnScanned`
  (params (SensorLevel :type Integer))
  (bind _malla (`self.Malla`))
  (set `self.bRevelada` true)
  (`SceneComponent.SetVisibility` (`self.Membrana`) true false)
  (`PrimitiveComponent.SetRenderCustomDepth` _malla true)
  (`PrimitiveComponent.SetCustomDepthStencilValue` _malla (`self.StencilEscaneo`))
  (`KismetSystemLibrary.K2_SetTimer` self "FinResaltado" 4.0))

(event `self.ReceiveActorBeginOverlap`
  (params (OtherActor :type "Actor Object Reference")))

(event `self.ReceiveTick`
  (params (DeltaSeconds :type "Float (single-precision)")))

(event `self.ReceiveAnyDamage`
  (params (Damage :type "Float (single-precision)") (DamageType :type "DamageType Object Reference") (InstigatedBy :type "Controller Object Reference") (DamageCauser :type "Actor Object Reference"))
  (`self.Explotar` self))

(event `self.Malla.OnComponentHit`
  (params (HitComponent :type "PrimitiveComponent Object Reference") (OtherActor :type "Actor Object Reference") (OtherComp :type "PrimitiveComponent Object Reference") (NormalImpulse :type "Vector Structure") (Hit :type "HitResult Structure (by ref)"))
  (bind _returnvalue (`PrimitiveComponent.GetPhysicsLinearVelocity` (`self.Malla`) "None"))
  (if (> (`KismetMathLibrary.VSize` _returnvalue) (`self.ImpactoMinimo`))
    (`self.Explotar` self)))

(event `/Game/EstacionNueve/Core/BPI_Interactuable.E_OnInteract`
  (params (InstigatorActor :type "Actor Object Reference")))

(event `/Game/EstacionNueve/Core/BPI_Interactuable.E_OnCompressed`)

(event `/Game/EstacionNueve/Core/BPI_Interactuable.E_OnDecompressed`
  (params (LaunchImpulse :type "Vector Structure")))

(event `/Game/EstacionNueve/Core/BPI_Interactuable.E_Fire`)

(event `/Game/EstacionNueve/Core/BPI_Interactuable.E_Reload`)

(event `/Game/EstacionNueve/Core/BPI_Interactuable.E_Hit`)

(fn `Explotar`
  (if (not (`self.bExplotado`))
    (set `self.bExplotado` true)
    (`GameplayStatics.ApplyRadialDamage` (`self.DanoExplosion`) (`self.K2_GetActorLocation` self) (`self.RadioExplosion`) "/Game/EstacionNueve/Core/DT_Explosion.DT_Explosion_C" (`|MakeArray` self :!type "Actor Object Reference") self null)
    (bind _asbp_gi_estacion_nueve (cast `/Game/EstacionNueve/Core/BP_GI_EstacionNueve` (`GameplayStatics.GetGameInstance` self)))
    (`/Game/EstacionNueve/Core/BP_GI_EstacionNueve.ReportNoise` _asbp_gi_estacion_nueve (`self.K2_GetActorLocation` self) (`self.RuidoExplosion`) "NewEnumerator5" self)
    (`self.K2_DestroyActor` self)))

(fn `FinResaltado`
  (bind _malla (`self.Malla`))
  (`PrimitiveComponent.SetRenderCustomDepth` _malla false)
  (`PrimitiveComponent.SetCustomDepthStencilValue` _malla 0))

(fn `GetInteractionPrompt`
  (returns (Prompt :type Text))
  (return ""))

(fn `UserConstructionScript`)