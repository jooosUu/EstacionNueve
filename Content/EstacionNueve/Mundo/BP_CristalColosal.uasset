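; Colossal stasis crystal that shatters from bullet or explosion damage or loud noise, releasing a creature if one is set.
; It listens to the GameInstance noise event, applying logarithmic distance falloff to decibels within a hearing radius.
; Romper runs once: it spawns the creature, sends a break notification and destroys the crystal.
; High-level scans briefly highlight the mesh through custom depth stencil.
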(event `self.ReceiveAnyDamage`
  (params (Damage :type "Float (single-precision)") (DamageType :type "DamageType Object Reference") (InstigatedBy :type "Controller Object Reference") (DamageCauser :type "Actor Object Reference"))
  (if (== (`GameplayStatics.GetObjectClass` DamageType) "/Game/EstacionNueve/Core/DT_Explosion.DT_Explosion_C")
    (`self.Romper`)
    (elif (== (`GameplayStatics.GetObjectClass` DamageType) "/Game/EstacionNueve/Core/DT_Bala.DT_Bala_C")
      (`self.Romper`))))

(event `OnNoiseRecibido`
  (params (Location :type "Vector Structure") (dB :type "Float (double-precision)") (Fuente :type "/Game/EstacionNueve/Core/E_NoiseSource Enum" :default "NewEnumerator0") (Instigador :type "Actor Object Reference"))
  (bind _returnvalue (`KismetMathLibrary.VSize` (- Location (`self.K2_GetActorLocation`))))
  (if (<= _returnvalue (`self.RadioEscucha`))
    (if (>= (- dB (* (/ (`KismetMathLibrary.Loge` (/ (`KismetMathLibrary.FMax` _returnvalue 100.0) 100.0)) (`KismetMathLibrary.Loge` 10.0)) 20.0)) (`self.UmbralPercibido`))
      (`self.Romper`))))

(event `self.E_OnScanned`
  (params (SensorLevel :type Integer))
  (if (>= SensorLevel 3)
    (`PrimitiveComponent.SetRenderCustomDepth` (`self.Malla`) true)
    (`PrimitiveComponent.SetCustomDepthStencilValue` (`self.Malla`) (`self.StencilEscaneo`))
    (`KismetSystemLibrary.K2_SetTimer` self "FinResaltado" 4.0)))

(event `self.ReceiveBeginPlay`
  (bind _asbp_gi_estacion_nueve (cast `/Game/EstacionNueve/Core/BP_GI_EstacionNueve` (`GameplayStatics.GetGameInstance`)))
  (add `/Game/EstacionNueve/Core/BP_GI_EstacionNueve.OnNoise` _asbp_gi_estacion_nueve (`|CreateDelegate` :!event `OnNoiseRecibido`)))

(fn `FinResaltado`
  (`PrimitiveComponent.SetRenderCustomDepth` (`self.Malla`) false))

(fn `GetInteractionPrompt`
  (returns (Prompt :type Text))
  (return ""))

(fn `Romper`
  (bind _clasecriatura (`self.ClaseCriatura`))
  (if (not (`self.bRoto`))
    (set `self.bRoto` true)
    (if (`KismetSystemLibrary.IsValidClass` _clasecriatura)
      (`|SpawnActorFromClass` _clasecriatura (`KismetMathLibrary.MakeTransform` (`self.K2_GetActorLocation`) (`self.K2_GetActorRotation`)) "AlwaysSpawn" "MultiplyWithRoot" null null))
    (bind _asbp_gi_estacion_nueve (cast `/Game/EstacionNueve/Core/BP_GI_EstacionNueve` (`GameplayStatics.GetGameInstance`)))
    (`/Game/EstacionNueve/Core/BP_GI_EstacionNueve.Notificar` _asbp_gi_estacion_nueve "Un cristal de estasis se ha roto")
    (`self.K2_DestroyActor`)))

(fn `UserConstructionScript`)