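; BP_TriggerZona is a zone trigger that acts as a checkpoint and announces the zone the player enters.
; When an actor tagged "Jugador" overlaps the Caja component, it stores the PuntoReaparicion world transform as the respawn point in BP_GI_EstacionNueve and passes NombreZona to that game instance's Notificar.
; It has no one-shot guard, so each qualifying overlap repeats both calls, and its interaction prompt is empty.
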(event `self.Caja.OnComponentBeginOverlap`
  (params (OverlappedComponent :type "PrimitiveComponent Object Reference") (OtherActor :type "Actor Object Reference") (OtherComp :type "PrimitiveComponent Object Reference") (OtherBodyIndex :type Integer) (bFromSweep :type Boolean) (SweepResult :type "HitResult Structure (by ref)"))
  (if (`self.ActorHasTag` OtherActor "Jugador")
    (bind _asbp_gi_estacion_nueve (cast `/Game/EstacionNueve/Core/BP_GI_EstacionNueve` (`GameplayStatics.GetGameInstance`)))
    (`/Game/EstacionNueve/Core/BP_GI_EstacionNueve.SetPuntoReaparicion` _asbp_gi_estacion_nueve (`SceneComponent.K2_GetComponentToWorld` (`self.PuntoReaparicion`)))
    (`/Game/EstacionNueve/Core/BP_GI_EstacionNueve.Notificar` _asbp_gi_estacion_nueve (`self.NombreZona`))))

(fn `GetInteractionPrompt`
  (returns (Prompt :type Text))
  (return ""))

(fn `UserConstructionScript`)