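; Sensor upgrade station that lets the interacting actor spend Mineral to raise its detector's sensor to level 2, then 3.
; On interaction it checks AC_Detector's level and AC_Inventario's stock, removes the cost and calls MejorarSensor.
; The interaction prompt repeats these checks on player 0's pawn, with cost amounts hardcoded in the text rather than read from the cost variables.
; Being scanned highlights the mesh through custom depth stencil for four seconds.
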(event `self.ReceiveBeginPlay`)

(event `/Game/EstacionNueve/Core/BPI_Interactuable.E_OnInteract`
  (params (InstigatorActor :type "Actor Object Reference"))
  (bind _costen2 (`self.CosteN2`))
  (bind _costen3 (`self.CosteN3`))
  (bind _asac_detector (cast `/Game/EstacionNueve/Componentes/AC_Detector` (`self.GetComponentByClass` InstigatorActor "/Game/EstacionNueve/Componentes/AC_Detector.AC_Detector_C")))
  (bind _asac_inventario (cast `/Game/EstacionNueve/Componentes/AC_Inventario` (`self.GetComponentByClass` InstigatorActor "/Game/EstacionNueve/Componentes/AC_Inventario.AC_Inventario_C")))
  (bind _sensorlevel (`/Game/EstacionNueve/Componentes/AC_Detector.SensorLevel` _asac_detector))
  (if (>= _sensorlevel 3)
    _
    (elif (== _sensorlevel 1)
      (bind _cantidad (`/Game/EstacionNueve/Componentes/AC_Inventario.GetCantidad` _asac_inventario "Mineral"))
      (if (>= _cantidad _costen2)
        (`/Game/EstacionNueve/Componentes/AC_Inventario.Quitar` _asac_inventario "Mineral" _costen2)
        (`/Game/EstacionNueve/Componentes/AC_Detector.MejorarSensor` _asac_detector))
      (elif (== _sensorlevel 2)
        (if (>= _cantidad _costen3)
          (`/Game/EstacionNueve/Componentes/AC_Inventario.Quitar` _asac_inventario "Mineral" _costen3)
          (`/Game/EstacionNueve/Componentes/AC_Detector.MejorarSensor` _asac_detector))))))

(event `self.ReceiveActorBeginOverlap`
  (params (OtherActor :type "Actor Object Reference")))

(event `self.ReceiveTick`
  (params (DeltaSeconds :type "Float (single-precision)")))

(event `/Game/EstacionNueve/Core/BPI_Interactuable.E_OnScanned`
  (params (SensorLevel :type Integer))
  (bind _malla (`self.Malla`))
  (`PrimitiveComponent.SetRenderCustomDepth` _malla true)
  (`PrimitiveComponent.SetCustomDepthStencilValue` _malla (`self.StencilEscaneo`))
  (`KismetSystemLibrary.K2_SetTimer` self "FinResaltado" 4.0))

(event `/Game/EstacionNueve/Core/BPI_Interactuable.E_OnCompressed`)

(event `/Game/EstacionNueve/Core/BPI_Interactuable.E_OnDecompressed`
  (params (LaunchImpulse :type "Vector Structure")))

(event `/Game/EstacionNueve/Core/BPI_Interactuable.E_Fire`)

(event `/Game/EstacionNueve/Core/BPI_Interactuable.E_Reload`)

(event `/Game/EstacionNueve/Core/BPI_Interactuable.E_Hit`)

(fn `FinResaltado`
  (`PrimitiveComponent.SetRenderCustomDepth` (`self.Malla`) false))

(fn `GetInteractionPrompt`
  (returns (Prompt :type Text))
  (bind _returnvalue (`GameplayStatics.GetPlayerPawn` self))
  (bind _asac_detector (cast `/Game/EstacionNueve/Componentes/AC_Detector` (`self.GetComponentByClass` _returnvalue "/Game/EstacionNueve/Componentes/AC_Detector.AC_Detector_C"))
    (:`then`
      (bind _asac_inventario (cast `/Game/EstacionNueve/Componentes/AC_Inventario` (`self.GetComponentByClass` _returnvalue "/Game/EstacionNueve/Componentes/AC_Inventario.AC_Inventario_C"))
        (:`then`
          (bind _sensorlevel (`/Game/EstacionNueve/Componentes/AC_Detector.SensorLevel` _asac_detector))
          (if (>= _sensorlevel 3)
            (return "")
            (elif (== _sensorlevel 1)
              (bind _cantidad (`/Game/EstacionNueve/Componentes/AC_Inventario.GetCantidad` _asac_inventario "Mineral"))
              (if (>= _cantidad (`self.CosteN2`))
                (return "Mejorar sensor a N2 (5 Mineral)")
                (else
                  (return "Necesitas 5 Mineral")))
              (elif (== _sensorlevel 2)
                (if (>= _cantidad (`self.CosteN3`))
                  (return "Mejorar sensor a N3 (10 Mineral)")
                  (else
                    (return "Necesitas 10 Mineral")))
                (else
                  (return ""))))))
        (:`CastFailed`
          (return ""))))
    (:`CastFailed`
      (return ""))))

(fn `UserConstructionScript`)