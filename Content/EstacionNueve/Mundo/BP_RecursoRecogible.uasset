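; BP_RecursoRecogible is a pickup resource actor that adds an item to the interacting actor's inventory.
; On interaction, it looks up the instigator's AC_Inventario component, passes its ItemID and Cantidad to Agregar, then destroys itself.
; Without that component nothing happens and the pickup stays in the world.
; GetInteractionPrompt builds a "Recoger" prompt text from the quantity and item ID.
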(event `self.E_OnInteract`
  (params (InstigatorActor :type "Actor Object Reference"))
  (bind _asac_inventario (cast `/Game/EstacionNueve/Componentes/AC_Inventario` (`self.GetComponentByClass` InstigatorActor "/Game/EstacionNueve/Componentes/AC_Inventario.AC_Inventario_C")))
  (`/Game/EstacionNueve/Componentes/AC_Inventario.Agregar` _asac_inventario (`self.ItemID`) (`self.Cantidad`))
  (`self.K2_DestroyActor`))

(fn `GetInteractionPrompt`
  (returns (Prompt :type Text))
  (return (`KismetTextLibrary.Conv_StringToText` (`KismetStringLibrary.Concat_StrStr` (`KismetStringLibrary.Concat_StrStr` (`KismetStringLibrary.Concat_StrStr` (`KismetStringLibrary.Concat_StrStr` "Recoger" " ") (`KismetStringLibrary.Conv_IntToString` (`self.Cantidad`))) " ") (`KismetStringLibrary.Conv_NameToString` (`self.ItemID`))))))

(fn `UserConstructionScript`)