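; BP_PuenteLevadizo is a drawbridge in EstacionNueve that lowers once, when an actor tagged Montura or Jugador enters its TriggerAterrizaje volume.
; The overlap sets a Bajado flag to block retriggering and sends a "Puente bajado" notification through the game instance.
; PuenteTimeline then drives the pitch of the Bisagra hinge component to swing the bridge.
; Other event stubs are empty, and the interaction prompt returns blank.
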(event `self.ReceiveBeginPlay`)

(event `self.TriggerAterrizaje.OnComponentBeginOverlap`
  (params (OverlappedComponent :type "PrimitiveComponent Object Reference") (OtherActor :type "Actor Object Reference") (OtherComp :type "PrimitiveComponent Object Reference") (OtherBodyIndex :type Integer) (bFromSweep :type Boolean) (SweepResult :type "HitResult Structure (by ref)"))
  (if (`self.bBajado`)
    _
    (elif (or (`self.ActorHasTag` OtherActor "Montura") (`self.ActorHasTag` OtherActor "Jugador"))
      (set `self.bBajado` true)
      (bind _asbp_gi_estacion_nueve (cast `/Game/EstacionNueve/Core/BP_GI_EstacionNueve` (`GameplayStatics.GetGameInstance`)))
      (`/Game/EstacionNueve/Core/BP_GI_EstacionNueve.Notificar` _asbp_gi_estacion_nueve "Puente bajado")
      (bind (_direction _pitch) (`Timeline|PuenteTimeline` :!via `PlayFromStart`)
        (:`Update`
          (`SceneComponent.K2_SetRelativeRotation` (`self.Bisagra`) (`KismetMathLibrary.MakeRotator` 0.0 _pitch) false false))))))

(event `self.ReceiveActorBeginOverlap`
  (params (OtherActor :type "Actor Object Reference")))

(event `self.ReceiveTick`
  (params (DeltaSeconds :type "Float (single-precision)")))

(fn `GetInteractionPrompt`
  (returns (Prompt :type Text))
  (return ""))

(fn `UserConstructionScript`)