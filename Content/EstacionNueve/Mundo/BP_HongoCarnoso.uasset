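; BP_HongoCarnoso is a harvestable fleshy mushroom pickup in the world that adds one HongoCarnoso item to the interacting actor's inventory.
; Interacting finds the AC_Inventario component on the instigator, calls Agregar, then hides the actor and sets a Recogido flag that blocks repeat pickups.
; A timer calls Reaparecer after a delay to show it again, and GetInteractionPrompt returns empty text while it is collected.
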(event `self.ReceiveBeginPlay`)

(event `/Game/EstacionNueve/Core/BPI_Interactuable.E_OnInteract`
  (params (InstigatorActor :type "Actor Object Reference"))
  (if (not (`self.bRecogido`))
    (bind _asac_inventario (cast `/Game/EstacionNueve/Componentes/AC_Inventario` (`self.GetComponentByClass` InstigatorActor "/Game/EstacionNueve/Componentes/AC_Inventario.AC_Inventario_C")))
    (`/Game/EstacionNueve/Componentes/AC_Inventario.Agregar` _asac_inventario "HongoCarnoso" 1)
    (set `self.bRecogido` true)
    (`self.SetActorHiddenInGame` self true)
    (`KismetSystemLibrary.K2_SetTimer` self "Reaparecer" 30.0)))

(event `self.ReceiveActorBeginOverlap`
  (params (OtherActor :type "Actor Object Reference")))

(event `self.ReceiveTick`
  (params (DeltaSeconds :type "Float (single-precision)")))

(event `/Game/EstacionNueve/Core/BPI_Interactuable.E_OnScanned`
  (params (SensorLevel :type Integer)))

(event `/Game/EstacionNueve/Core/BPI_Interactuable.E_OnCompressed`)

(event `/Game/EstacionNueve/Core/BPI_Interactuable.E_OnDecompressed`
  (params (LaunchImpulse :type "Vector Structure")))

(event `/Game/EstacionNueve/Core/BPI_Interactuable.E_Fire`)

(event `/Game/EstacionNueve/Core/BPI_Interactuable.E_Reload`)

(event `/Game/EstacionNueve/Core/BPI_Interactuable.E_Hit`)

(fn `GetInteractionPrompt`
  (returns (Prompt :type Text))
  (locals (PromptText :type Text))
  (if (`self.bRecogido`)
    (set `local.PromptText` "")
    (else
      (set `local.PromptText` "Recoger Hongo Carnoso")))
  (return (`local.PromptText`)))

(fn `Reaparecer`
  (`self.SetActorHiddenInGame` self false)
  (set `self.bRecogido` false))

(fn `UserConstructionScript`)