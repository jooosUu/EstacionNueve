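; BP_NodoExcavable is a minable rock node that stays locked until an Eon scan of sufficient sensor level reveals its vein.
; Construction sets required level and health from TipoNodo (Basico, Diamante, Ambar).
; Scans show the matching vein and briefly highlight the mesh via custom depth stencil.
; Only DT_Pico damage depletes revealed nodes, granting AC_Inventario items or spawning BP_AmbarExtraible; hitting hidden nodes triggers a throttled "scan first" notification.
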(event `self.ReceiveBeginPlay`)

(event `/Game/EstacionNueve/Core/BPI_Interactuable.E_OnScanned`
  (params (SensorLevel :type Integer))
  (bind _malla (`self.Malla`))
  (bind _tiponodo (`self.TipoNodo`))
  (if (>= SensorLevel (`self.NivelRequerido`))
    (`|ExecutionSequence`
      (:`then_0`
        (if (not (`self.bRevelado`))
          (`|ExecutionSequence`
            (:`then_0`
              (set `self.bRevelado` true)
              (if (`|EnumEquality` _tiponodo "NewEnumerator0")
                (`SceneComponent.SetVisibility` (`self.VetaCian`) true false)
                (`SceneComponent.SetVisibility` (`self.VetaBlanca`) false false)
                (`SceneComponent.SetVisibility` (`self.VetaNaranja`) false false)))
            (:`then_1`
              (if (`|EnumEquality` _tiponodo "NewEnumerator1")
                (`SceneComponent.SetVisibility` (`self.VetaBlanca`) true false)
                (`SceneComponent.SetVisibility` (`self.VetaCian`) false false)
                (`SceneComponent.SetVisibility` (`self.VetaNaranja`) false false)))
            (:`then_2`
              (if (`|EnumEquality` _tiponodo "NewEnumerator2")
                (`SceneComponent.SetVisibility` (`self.VetaNaranja`) true false)
                (`SceneComponent.SetVisibility` (`self.VetaCian`) false false)
                (`SceneComponent.SetVisibility` (`self.VetaBlanca`) false false))))))
      (:`then_1`
        (`PrimitiveComponent.SetRenderCustomDepth` _malla true)
        (`PrimitiveComponent.SetCustomDepthStencilValue` _malla (`self.StencilEscaneo`))
        (`KismetSystemLibrary.K2_SetTimerDelegate` (delegate `FinResaltado`) 4.0)))))

(event `FinResaltado`
  (`PrimitiveComponent.SetRenderCustomDepth` (`self.Malla`) false))

(event `self.ReceiveActorBeginOverlap`
  (params (OtherActor :type "Actor Object Reference")))

(event `self.ReceiveTick`
  (params (DeltaSeconds :type "Float (single-precision)")))

(event `FinAviso`
  (set `self.bAvisoReciente` false))

(event `self.ReceiveAnyDamage`
  (params (Damage :type "Float (single-precision)") (DamageType :type "DamageType Object Reference") (InstigatedBy :type "Controller Object Reference") (DamageCauser :type "Actor Object Reference"))
  (if (`self.bRevelado`)
    (cast `/Game/EstacionNueve/Core/DT_Pico` DamageType)
    (set `self.Vida` (- (`self.Vida`) Damage))
    (if (<= (`self.Vida`) 0.0)
      (`self.Muerte` InstigatedBy))
    (elif (not (`self.bAvisoReciente`))
      (bind _asbp_gi_estacion_nueve (cast `/Game/EstacionNueve/Core/BP_GI_EstacionNueve` (`GameplayStatics.GetGameInstance`)))
      (`/Game/EstacionNueve/Core/BP_GI_EstacionNueve.Notificar` _asbp_gi_estacion_nueve "Roca sólida: escanea primero")
      (set `self.bAvisoReciente` true)
      (`KismetSystemLibrary.K2_SetTimerDelegate` (delegate `FinAviso`) 5.0))))

(event `Muerte`
  (params (InstigatedBy :type "Controller Object Reference"))
  (bind _tiponodo (`self.TipoNodo`))
  (`|ExecutionSequence`
    (:`then_0`
      (if (`|EnumEquality` _tiponodo "NewEnumerator0")
        (`self.DarItem` InstigatedBy "Mineral" 2)))
    (:`then_1`
      (if (`|EnumEquality` _tiponodo "NewEnumerator1")
        (`self.DarItem` InstigatedBy "Diamante" 1)))
    (:`then_2`
      (if (`|EnumEquality` _tiponodo "NewEnumerator2")
        (`|SpawnActorFromClass` "/Game/EstacionNueve/Mundo/BP_AmbarExtraible.BP_AmbarExtraible_C" (`KismetMathLibrary.MakeTransform` (`self.K2_GetActorLocation` self) (`self.K2_GetActorRotation` self) (`KismetMathLibrary.MakeVector` 1.0 1.0 1.0)) "Undefined" "SelectDefaultAtRuntime" null null)
        (`self.K2_DestroyActor` self)))))

(event `DarItem`
  (params (InstigatedBy :type "Controller Object Reference") (ItemID :type Name) (Cantidad :type Integer))
  (bind _asac_inventario (cast `/Game/EstacionNueve/Componentes/AC_Inventario` (`self.GetComponentByClass` (`Controller.K2_GetPawn` InstigatedBy) "/Game/EstacionNueve/Componentes/AC_Inventario.AC_Inventario_C")))
  (`/Game/EstacionNueve/Componentes/AC_Inventario.Agregar` _asac_inventario ItemID Cantidad)
  (`self.K2_DestroyActor` self))

(event `/Game/EstacionNueve/Core/BPI_Interactuable.E_OnInteract`
  (params (InstigatorActor :type "Actor Object Reference")))

(event `/Game/EstacionNueve/Core/BPI_Interactuable.E_OnCompressed`)

(event `/Game/EstacionNueve/Core/BPI_Interactuable.E_OnDecompressed`
  (params (LaunchImpulse :type "Vector Structure")))

(event `/Game/EstacionNueve/Core/BPI_Interactuable.E_Fire`)

(event `/Game/EstacionNueve/Core/BPI_Interactuable.E_Reload`)

(event `/Game/EstacionNueve/Core/BPI_Interactuable.E_Hit`)

(fn `GetInteractionPrompt`
  (returns (Prompt :type Text))
  (return (`KismetTextLibrary.Conv_StringToText` "Excavar [Pico]")))

(fn `UserConstructionScript`
  (switch `/Game/EstacionNueve/Core/E_TipoNodo` (`self.TipoNodo`)
    (:`NewEnumerator0`
      (set `self.NivelRequerido` 1)
      (set `self.Vida` 60.0))
    (:`NewEnumerator1`
      (set `self.NivelRequerido` 2)
      (set `self.Vida` 100.0))
    (:`NewEnumerator2`
      (set `self.NivelRequerido` 2)
      (set `self.Vida` 80.0))))