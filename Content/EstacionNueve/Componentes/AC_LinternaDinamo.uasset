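; AC_LinternaDinamo is an actor component for a dynamo flashlight that must be pumped to stay lit.
; On BeginPlay it finds the owner's SpotLightComponent and tints it warm amber.
; While the light is visible, Tick drains Carga and scales intensity from it, adding random flicker near or below UmbralParpadeo.
; Bombear adds charge up to full, rate-limited by IntervaloBombeo, and records acceptance in BombeoAceptado.
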(event `self.ReceiveBeginPlay`
  (set `self.Lampara` (`Actor.GetComponentByClass` (`self.GetOwner`) "/Script/Engine.SpotLightComponent"))
  (`LightComponent.SetLightColor` (`self.Lampara`) (struct :`R` 1.0 :`G` 0.78 :`B` 0.42 :`A` 1.0) true))

(event `self.ReceiveTick`
  (params (DeltaSeconds :type "Float (single-precision)"))
  (bind _lampara (`self.Lampara`))
  (bind _returnvalue (`KismetMathLibrary.FMax` (- (`self.Carga`) (/ DeltaSeconds (`self.DuracionSegundos`)))))
  (if (`KismetSystemLibrary.IsValid` _lampara)
    (if (`SceneComponent.IsVisible` _lampara)
      (set `self.Carga` _returnvalue)
      (`LightComponent.SetIntensity` _lampara (* (* (`self.IntensidadMaxima`) (`KismetMathLibrary.FClamp` (* _returnvalue 1.6))) (`KismetMathLibrary.FMax` (`KismetMathLibrary.RandomFloatInRange` 0.45 1.0) (`KismetMathLibrary.FClamp` (* (- _returnvalue (`self.UmbralParpadeo`)) 100.0))))))))

(event `Bombear`
  (bind _returnvalue (`GameplayStatics.GetTimeSeconds`))
  (bind _returnvalue_2 (>= (- _returnvalue (`self.UltimoBombeo`)) (`self.IntervaloBombeo`)))
  (set `self.bBombeoAceptado` _returnvalue_2)
  (if _returnvalue_2
    (set `self.UltimoBombeo` _returnvalue)
    (set `self.Carga` (`KismetMathLibrary.FMin` (+ (`self.Carga`) (`self.CargaPorBombeo`)) 1.0))))