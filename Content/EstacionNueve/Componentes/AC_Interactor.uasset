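; Actor component that handles interaction targeting and a toggleable spotlight lamp for its owner.
; A looping timer, rather than Tick, line-traces from the owner's camera for BPI_Interactuable actors, caching the target for Interactuar to message.
; Prompt text comes from the target, overridden when tagged Composable or Excavable targets need another tool from AC_Inventario.
; Dispatchers report lamp toggles and prompt changes, though every prompt broadcast passes hidden, empty values.
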(event `self.ReceiveBeginPlay`
  (set `self.Lampara` (`Actor.GetComponentByClass` (`self.GetOwner`) "/Script/Engine.SpotLightComponent"))
  (bind _returnvalue (`KismetSystemLibrary.K2_SetTimer` self "ActualizarObjetivo" 0.1 true))
  (set `self.TimerObjetivo` _returnvalue))

(event `self.ReceiveTick`
  (params (DeltaSeconds :type "Float (single-precision)")))

(fn `ActualizarObjetivo`
  (locals (TextoNuevo :type Text) (UbicacionCamara :type "Vector Structure") (DireccionCamara :type "Vector Structure"))
  (bind _returnvalue (`self.GetOwner`))
  (bind _ubicacioncamara (`local.UbicacionCamara`))
  (bind _textonuevo (`local.TextoNuevo`))
  (bind _objetivoactual (`self.ObjetivoActual`))
  (bind _returnvalue_2 (`Actor.GetComponentByClass` _returnvalue "/Script/Engine.CameraComponent"))
  (bind _returnvalue_3 (`Actor.GetComponentByClass` _returnvalue "/Game/EstacionNueve/Componentes/AC_Inventario.AC_Inventario_C"))
  (bind _returnvalue_4 (`KismetSystemLibrary.IsValid` _returnvalue_3))
  (bind _herramientaequipada (`/Game/EstacionNueve/Componentes/AC_Inventario.HerramientaEquipada` _returnvalue_3))
  (set `local.UbicacionCamara` (`SceneComponent.K2_GetComponentLocation` _returnvalue_2))
  (set `local.DireccionCamara` (`SceneComponent.GetForwardVector` _returnvalue_2))
  (bind (_outhit _returnvalue_5) (`KismetSystemLibrary.LineTraceSingle` _ubicacioncamara (+ (* (`local.DireccionCamara`) (`self.RangoInteraccion`)) _ubicacioncamara) "TraceTypeQuery1"))
  (if _returnvalue_5
    (bind (_bblockinghit _binitialoverlap _time _distance _location _impactpoint _normal _impactnormal _physmat _hitactor) (`GameplayStatics.BreakHitResult` _outhit))
    (if (`KismetSystemLibrary.DoesImplementInterface` _hitactor "/Game/EstacionNueve/Core/BPI_Interactuable.BPI_Interactuable_C")
      (`|ExecutionSequence`
        (:`then_0`
          (set `self.ObjetivoActual` _hitactor)
          (bind _prompt (message `/Game/EstacionNueve/Core/BPI_Interactuable.GetInteractionPrompt` _hitactor))
          (if _returnvalue_4
            (if (and (and _returnvalue_4 (`|EnumInequality` _herramientaequipada (enumliteral `/Game/EstacionNueve/Core/E_EquippedTool` "NewEnumerator1"))) (`Actor.ActorHasTag` _objetivoactual "Composable"))
              (set `local.TextoNuevo` "Necesitas el Rayo Compresor [1]")
              (elif (and (and _returnvalue_4 (`|EnumInequality` _herramientaequipada (enumliteral `/Game/EstacionNueve/Core/E_EquippedTool` "NewEnumerator2"))) (`Actor.ActorHasTag` _objetivoactual "Excavable"))
                (set `local.TextoNuevo` "Necesitas el Pico")
                (else
                  (set `local.TextoNuevo` _prompt))))
            (else
              (set `local.TextoNuevo` _prompt))))
        (:`then_1`
          (if (`KismetTextLibrary.NotEqual_TextText` _textonuevo (`self.TextoActual`))
            (set `self.TextoActual` _textonuevo)
            (`self.OnPromptCambiado` false))))
      (elif (`KismetSystemLibrary.IsValid` (`self.ObjetivoActual`))
        (set `self.ObjetivoActual` null)
        (`self.OnPromptCambiado` false)))
    (elif (`KismetSystemLibrary.IsValid` (`self.ObjetivoActual`))
      (set `self.ObjetivoActual` null)
      (`self.OnPromptCambiado` false))))

(fn `AlternarLampara`
  (bind _blamparaencendida (`self.bLamparaEncendida`))
  (bind _lampara (`self.Lampara`))
  (set `self.bLamparaEncendida` (not (`self.bLamparaEncendida`)))
  (if (`KismetSystemLibrary.IsValid` _lampara)
    (`SceneComponent.SetVisibility` _lampara (`self.bLamparaEncendida`) false)
    (`self.OnLamparaCambiada` _blamparaencendida)
    (else
      (`self.OnLamparaCambiada` _blamparaencendida))))

(fn `Interactuar`
  (bind _objetivoactual (`self.ObjetivoActual`))
  (if (`KismetSystemLibrary.IsValid` _objetivoactual)
    (message `/Game/EstacionNueve/Core/BPI_Interactuable.E_OnInteract` _objetivoactual (`self.GetOwner` self))))