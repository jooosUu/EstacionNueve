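; Inventory component with three stores: limited compressed-item slots, quantity-based pockets and unlockable tools.
; Compressed items come out last-in first or by ID, and each change broadcasts slot count and summed noise penalty in dB.
; Pockets map item IDs to quantities, refusing removals beyond stock and dropping emptied entries.
; Equipping accepts only unlocked tools or the default enum entry; pocket and equip changes also fire dispatchers.
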(fn `Agregar`
  (params (ItemID :type Name) (Cantidad :type Integer))
  (bind _returnvalue (+ (`self.GetCantidad` self ItemID) Cantidad))
  (`BlueprintMapLibrary.Map_Add` (`self.Bolsillos`) ItemID _returnvalue)
  (`self.OnBolsillosCambiado` self ItemID _returnvalue))

(fn `DesbloquearHerramienta`
  (params (T :type "/Game/EstacionNueve/Core/E_EquippedTool Enum" :default "NewEnumerator0"))
  (if (not (`KismetArrayLibrary.Array_Contains` (`self.HerramientasDesbloqueadas`) T))
    (`KismetArrayLibrary.Array_AddUnique` (`self.HerramientasDesbloqueadas`) T)))

(fn `EquiparHerramienta`
  (params (T :type "/Game/EstacionNueve/Core/E_EquippedTool Enum" :default "NewEnumerator0"))
  (returns (bExito :type Boolean))
  (bind _returnvalue (or (`|EnumEquality` T "E_EquippedTool::NewEnumerator0") (`self.EstaDesbloqueada` T)))
  (if _returnvalue
    (set `self.HerramientaEquipada` T)
    (`self.OnHerramientaCambiada` T)
    (return _returnvalue)))

(fn `EstaDesbloqueada`
  (params (T :type "/Game/EstacionNueve/Core/E_EquippedTool Enum" :default "NewEnumerator0"))
  (returns (bDesbloqueada :type Boolean))
  (return (`KismetArrayLibrary.Array_Contains` (`self.HerramientasDesbloqueadas`) T)))

(fn `GetCantidad`
  (params (ItemID :type Name))
  (returns (Cantidad :type Integer))
  (return (`BlueprintMapLibrary.Map_Find` (`self.Bolsillos`) ItemID)))

(fn `GetNumComprimidos`
  (returns (Num :type Integer))
  (return (`KismetArrayLibrary.Array_Length` (`self.SlotsComprimidos`))))

(fn `GetRuidoComprimidos`
  (returns (Ruido :type "Float (single-precision)"))
  (locals (TotalRuido :type "Float (single-precision)" :default 0.0))
  (for _array_element (`self.SlotsComprimidos`)
    (set `local.TotalRuido` (+ (`local.TotalRuido`) (`.NoisePenalty_dB_10_C389ADC3469C1F28D4C443835029FF04` (break `/Game/EstacionNueve/Core/FItemStruct` _array_element)))))
  (return (`local.TotalRuido`)))

(fn `GuardarComprimido`
  (params (Item :type "/Game/EstacionNueve/Core/FItemStruct Structure"))
  (returns (bGuardado :type Boolean))
  (locals (bResultado :type Boolean :default false))
  (if (`self.HayEspacioComprimido` self)
    (`KismetArrayLibrary.Array_Add` (`self.SlotsComprimidos`) Item)
    (`self.OnComprimidosCambiado` (`self.GetNumComprimidos` self) (`self.GetRuidoComprimidos` self))
    (set `local.bResultado` true))
  (return (`local.bResultado`)))

(fn `HayEspacioComprimido`
  (returns (bHay :type Boolean))
  (return (< (`KismetArrayLibrary.Array_Length` (`self.SlotsComprimidos`)) (`self.MaxSlots`))))

(fn `Quitar`
  (params (ItemID :type Name) (Cantidad :type Integer))
  (returns (bExito :type Boolean))
  (bind _cantidad (`self.GetCantidad` self ItemID))
  (bind _returnvalue (- _cantidad Cantidad))
  (if (< _cantidad Cantidad)
    (return false)
    (elif (<= _returnvalue 0)
      (`BlueprintMapLibrary.Map_Remove` (`self.Bolsillos`) ItemID)
      (`self.OnBolsillosCambiado` self ItemID 0)
      (return true)
      (else
        (`BlueprintMapLibrary.Map_Add` (`self.Bolsillos`) ItemID _returnvalue)
        (`self.OnBolsillosCambiado` self ItemID _returnvalue)
        (return true)))))

(fn `SacarComprimidoPorID`
  (params (ItemID :type Name))
  (returns (bExito :type Boolean) (Item :type "/Game/EstacionNueve/Core/FItemStruct Structure"))
  (locals (bResultado :type Boolean :default false) (IndiceEncontrado :type Integer :default -1) (ItemLocal :type "/Game/EstacionNueve/Core/FItemStruct Structure"))
  (bind _indiceencontrado (`local.IndiceEncontrado`))
  (for (_array_element _array_index) (`self.SlotsComprimidos`)
    (if (and (== (`.ItemID_6_0EDF8A2C4803C10EBED9C7ACCFEF82E7` (break `/Game/EstacionNueve/Core/FItemStruct` _array_element)) ItemID) (< _indiceencontrado 0))
      (set `local.ItemLocal` _array_element)
      (set `local.IndiceEncontrado` _array_index)))
  (if (>= _indiceencontrado 0)
    (`KismetArrayLibrary.Array_Remove` (`self.SlotsComprimidos`) (`local.IndiceEncontrado`))
    (`self.OnComprimidosCambiado` (`self.GetNumComprimidos` self) (`self.GetRuidoComprimidos` self))
    (set `local.bResultado` true))
  (return (`local.bResultado`) (`local.ItemLocal`)))

(fn `SacarUltimoComprimido`
  (returns (bExito :type Boolean) (Item :type "/Game/EstacionNueve/Core/FItemStruct Structure"))
  (locals (bResultado :type Boolean :default false) (IndiceAExtraer :type Integer :default 0) (ItemLocal :type "/Game/EstacionNueve/Core/FItemStruct Structure"))
  (bind _slotscomprimidos (`self.SlotsComprimidos`))
  (if (> (`KismetArrayLibrary.Array_Length` (`self.SlotsComprimidos`)) 0)
    (set `local.IndiceAExtraer` (- (`KismetArrayLibrary.Array_Length` _slotscomprimidos) 1))
    (set `local.ItemLocal` (`|GetArrayItem` _slotscomprimidos (`local.IndiceAExtraer`)))
    (`KismetArrayLibrary.Array_Remove` (`self.SlotsComprimidos`) (`local.IndiceAExtraer`))
    (`self.OnComprimidosCambiado` (`self.GetNumComprimidos`) (`self.GetRuidoComprimidos`))
    (set `local.bResultado` true))
  (return (`local.bResultado`) (`local.ItemLocal`)))

(fn `Tiene`
  (params (ItemID :type Name) (Cantidad :type Integer))
  (returns (bTiene :type Boolean))
  (return (>= (`self.GetCantidad` ItemID) Cantidad)))