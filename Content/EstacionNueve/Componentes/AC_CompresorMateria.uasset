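; Actor component for a matter compressor ray that shrinks "Composable" objects into the owner's inventory and launches them back out.
; Comprimir targets the interactor's object or a camera trace, matches its DT_ItemsComprimibles row, then shrinks, stores and destroys it.
; Lanzar respawns the last stored item with an impulse, briefly ignoring owner collision.
; A looping timer lerps scale and holds a busy lock; both actions report noise to AC_Detector.
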(event `self.ReceiveBeginPlay`
  (set `self.Inventario` (`Actor.GetComponentByClass` (`self.GetOwner`) "/Game/EstacionNueve/Componentes/AC_Inventario.AC_Inventario_C"))
  (set `self.Detector` (`Actor.GetComponentByClass` (`self.GetOwner`) "/Game/EstacionNueve/Componentes/AC_Detector.AC_Detector_C")))

(event `self.ReceiveTick`
  (params (DeltaSeconds :type "Float (single-precision)")))

(fn `ActualizarEscala`
  (bind _alphaescala (`self.AlphaEscala`))
  (bind _actorescalando (`self.ActorEscalando`))
  (bind (_itemid _itemclass _originalscale _biscompressed _noisepenalty_db) (break `/Game/EstacionNueve/Core/FItemStruct` (`self.FilaGuardada`)))
  (`|ExecutionSequence`
    (:`then_0`
      (set `self.AlphaEscala` (+ (`self.AlphaEscala`) (/ 0.02 (`self.Duracion`))))
      (if (`KismetSystemLibrary.IsValid` _actorescalando)
        (`Actor.SetActorScale3D` _actorescalando (`KismetMathLibrary.VLerp` (`self.EscalaDesde`) (`self.EscalaHasta`) _alphaescala))
        (else
          (`KismetSystemLibrary.K2_ClearAndInvalidateTimerHandle` (`self.TimerEscala`))
          (set `self.bOcupado` false)
          (set `self.AlphaEscala` 0.0))))
    (:`then_1`
      (if (>= _alphaescala 1.0)
        (`KismetSystemLibrary.K2_ClearAndInvalidateTimerHandle` (`self.TimerEscala`))
        (set `self.bOcupado` false)
        (if (`self.bModoComprimir`)
          (`/Game/EstacionNueve/Componentes/AC_Inventario.GuardarComprimido` (`self.Inventario`) (make `/Game/EstacionNueve/Core/FItemStruct` _itemid _itemclass (`self.EscalaOriginal`) true _noisepenalty_db))
          (`/Game/EstacionNueve/Componentes/AC_Detector.ReportarRuidoPuntual` (`self.Detector`) 15.0 (enumliteral `/Game/EstacionNueve/Core/E_NoiseSource` "NewEnumerator1"))
          (`Actor.K2_DestroyActor` _actorescalando)
          (set `self.ActorEscalando` null))))))

(fn `Comprimir`
  (locals (bEncontrada :type Boolean :default false) (ActorObjetivo :type "Actor Object Reference") (UbicacionCamara :type "Vector Structure") (ForwardCamara :type "Vector Structure"))
  (bind _returnvalue (`GameplayStatics.GetGameInstance`))
  (bind _actorobjetivo (`local.ActorObjetivo`))
  (bind _returnvalue_2 (`Actor.GetActorScale3D` _actorobjetivo))
  (bind _returnvalue_3 (`Actor.GetActorScale3D` _actorobjetivo))
  (bind _returnvalue_4 (`Actor.GetComponentByClass` (`self.GetOwner`) "/Script/Engine.CameraComponent"))
  (bind _returnvalue_5 (`GameplayStatics.GetObjectClass` _actorobjetivo))
  (bind _returnvalue_6 (`SceneComponent.K2_GetComponentLocation` _returnvalue_4))
  (bind _returnvalue_7 (`KismetMathLibrary.GetForwardVector` (`SceneComponent.K2_GetComponentRotation` _returnvalue_4)))
  (if (not (`self.bOcupado`))
    (bind _asac_interactor (cast `/Game/EstacionNueve/Componentes/AC_Interactor` (`Actor.GetComponentByClass` (`self.GetOwner`) "/Game/EstacionNueve/Componentes/AC_Interactor.AC_Interactor_C"))
      (:`then`
        (bind _objetivoactual (`/Game/EstacionNueve/Componentes/AC_Interactor.ObjetivoActual` _asac_interactor))
        (`/Engine/EditorBlueprintResources/StandardMacros.IsValid` _objetivoactual
          (:`Is Valid`
            (if (`Actor.ActorHasTag` _objetivoactual "Composable")
              (set `local.ActorObjetivo` _objetivoactual)
              (`/Engine/EditorBlueprintResources/StandardMacros.IsValid` _actorobjetivo :!label _label
                (:`Is Valid`
                  (if (`Actor.ActorHasTag` _actorobjetivo "Composable")
                    (if (`/Game/EstacionNueve/Componentes/AC_Inventario.HayEspacioComprimido` (`self.Inventario`))
                      (bind _outrownames (`DataTableFunctionLibrary.GetDataTableRowNames` "/Game/EstacionNueve/Core/DT_ItemsComprimibles.DT_ItemsComprimibles"))
                      (for _array_element _outrownames
                        (bind _returnvalue_8 (`|GetDataTableRow` "/Game/EstacionNueve/Core/DT_ItemsComprimibles.DT_ItemsComprimibles" _array_element)
                          (:`then`
                            (if (== (`.ItemClass_7_C00B6E6048109AD974D66A8B097E56A3` (break `/Game/EstacionNueve/Core/FItemStruct` _returnvalue_8)) _returnvalue_5)
                              (set `self.FilaGuardada` _returnvalue_8)
                              (set `local.bEncontrada` true)
                              (break)))))
                      (if (not (`local.bEncontrada`))
                        (set `self.FilaGuardada` (make `/Game/EstacionNueve/Core/FItemStruct` (`KismetStringLibrary.Conv_StringToName` (`KismetSystemLibrary.GetClassDisplayName` _returnvalue_5)) _returnvalue_5 _returnvalue_2 true 5.0)))
                      (message `/Game/EstacionNueve/Core/BPI_Interactuable.E_OnCompressed` _actorobjetivo)
                      (bind _asprimitive_component (cast `PrimitiveComponent` (`Actor.GetComponentByClass` _actorobjetivo "/Script/Engine.PrimitiveComponent")))
                      (`PrimitiveComponent.SetSimulatePhysics` _asprimitive_component false)
                      (`PrimitiveComponent.SetCollisionEnabled` _asprimitive_component "NoCollision")
                      (set `self.EscalaOriginal` _returnvalue_2)
                      (set `self.bOcupado` true)
                      (set `self.ActorEscalando` _actorobjetivo)
                      (set `self.EscalaDesde` _returnvalue_3)
                      (set `self.EscalaHasta` (* _returnvalue_3 (`self.EscalaMinima`)))
                      (set `self.Duracion` (`self.TiempoCompresion`))
                      (set `self.AlphaEscala` 0.0)
                      (set `self.bModoComprimir` true)
                      (bind _returnvalue_9 (`KismetSystemLibrary.K2_SetTimer` self "ActualizarEscala" 0.02 true))
                      (set `self.TimerEscala` _returnvalue_9)
                      (else
                        (bind _asbp_gi_estacion_nueve (cast `/Game/EstacionNueve/Core/BP_GI_EstacionNueve` _returnvalue))
                        (`/Game/EstacionNueve/Core/BP_GI_EstacionNueve.Notificar` _asbp_gi_estacion_nueve (`KismetTextLibrary.Conv_StringToText` "Bolso lleno (3/3)"))))
                    (else
                      (bind _asbp_gi_estacion_nueve_2 (cast `/Game/EstacionNueve/Core/BP_GI_EstacionNueve` _returnvalue))
                      (`/Game/EstacionNueve/Core/BP_GI_EstacionNueve.Notificar` _asbp_gi_estacion_nueve_2 (`KismetTextLibrary.Conv_StringToText` "Este objeto no se puede comprimir"))))))
              (else
                (set `local.UbicacionCamara` _returnvalue_6 :!label _label_2)
                (set `local.ForwardCamara` _returnvalue_7)
                (bind (_outhit _returnvalue_10) (`KismetSystemLibrary.LineTraceSingle` :`Start` _returnvalue_6 :`End` (+ _returnvalue_6 (* _returnvalue_7 (`self.Rango`))) :`TraceChannel` (enumliteral `ETraceTypeQuery` "TraceTypeQuery1") :`DrawDebugType` (enumliteral `EDrawDebugTrace` "None")))
                (if _returnvalue_10
                  (set `local.ActorObjetivo` (`.HitActor` (`GameplayStatics.BreakHitResult` _outhit)))
                  (goto _label)
                  (else
                    (bind _asbp_gi_estacion_nueve_3 (cast `/Game/EstacionNueve/Core/BP_GI_EstacionNueve` _returnvalue))
                    (`/Game/EstacionNueve/Core/BP_GI_EstacionNueve.Notificar` _asbp_gi_estacion_nueve_3 "El rayo no alcanza nada"))))))
          (:`Is Not Valid`
            (goto _label_2))))
      (:`CastFailed`
        (goto _label_2)))
    (else
      (bind _asbp_gi_estacion_nueve_4 (cast `/Game/EstacionNueve/Core/BP_GI_EstacionNueve` _returnvalue))
      (`/Game/EstacionNueve/Core/BP_GI_EstacionNueve.Notificar` _asbp_gi_estacion_nueve_4 "El rayo se esta recargando"))))

(fn `Lanzar`
  (locals (ForwardDueno :type "Vector Structure") (OrigenSpawn :type "Vector Structure"))
  (bind _returnvalue (`self.GetOwner`))
  (bind _returnvalue_2 (`Actor.GetActorForwardVector` _returnvalue))
  (bind _returnvalue_3 (`Actor.K2_GetActorLocation` _returnvalue))
  (bind _returnvalue_4 (* _returnvalue_2 (`self.Impulso`)))
  (if (`self.bOcupado`)
    (bind _asbp_gi_estacion_nueve (cast `/Game/EstacionNueve/Core/BP_GI_EstacionNueve` (`GameplayStatics.GetGameInstance`)))
    (`/Game/EstacionNueve/Core/BP_GI_EstacionNueve.Notificar` _asbp_gi_estacion_nueve "El rayo se esta recargando")
    (else
      (bind (_bexito _item) (`/Game/EstacionNueve/Componentes/AC_Inventario.SacarUltimoComprimido` (`self.Inventario`)))
      (if _bexito
        (set `local.ForwardDueno` _returnvalue_2)
        (set `local.OrigenSpawn` _returnvalue_3)
        (bind (_itemid _itemclass _originalscale) (break `/Game/EstacionNueve/Core/FItemStruct` _item))
        (bind _returnvalue_5 (`|SpawnActorFromClass` _itemclass (`KismetMathLibrary.MakeTransform` (+ _returnvalue_3 (* _returnvalue_2 (`self.DistanciaAparicion`))) (`Actor.K2_GetActorRotation` _returnvalue)) "AlwaysSpawn" "MultiplyWithRoot" null null))
        (if (`KismetSystemLibrary.IsValid` _returnvalue_5)
          (set `self.ActorLanzado` _returnvalue_5)
          (`Actor.SetActorScale3D` _returnvalue_5 (* _originalscale (`self.EscalaMinima`)))
          (bind _asprimitive_component (cast `PrimitiveComponent` (`Actor.K2_GetRootComponent` _returnvalue_5)))
          (`PrimitiveComponent.IgnoreActorWhenMoving` _asprimitive_component _returnvalue true)
          (bind _returnvalue_6 (`KismetSystemLibrary.K2_SetTimer` null "LiberarIgnorarDueno" 0.5))
          (set `self.Temporizador` _returnvalue_6)
          (message `/Game/EstacionNueve/Core/BPI_Interactuable.E_OnDecompressed` _returnvalue_5 _returnvalue_4)
          (`PrimitiveComponent.AddImpulse` _asprimitive_component _returnvalue_4 "None" true)
          (set `self.bOcupado` true)
          (set `self.ActorEscalando` _returnvalue_5)
          (set `self.EscalaDesde` (`Actor.GetActorScale3D` _returnvalue_5))
          (set `self.EscalaHasta` _originalscale)
          (set `self.Duracion` (`self.TiempoExpansion`))
          (set `self.AlphaEscala` 0.0)
          (set `self.bModoComprimir` false)
          (bind _returnvalue_7 (`KismetSystemLibrary.K2_SetTimer` null "ActualizarEscala" 0.02 true))
          (set `self.TimerEscala` _returnvalue_7)
          (`/Game/EstacionNueve/Componentes/AC_Detector.ReportarRuidoPuntual` (`self.Detector`) 20.0 (enumliteral `/Game/EstacionNueve/Core/E_NoiseSource` "NewEnumerator4")))))))

(fn `LiberarIgnorarDueno`
  (bind _actorlanzado (`self.ActorLanzado`))
  (if (`KismetSystemLibrary.IsValid` _actorlanzado)
    (bind _asprimitive_component (cast `PrimitiveComponent` (`Actor.K2_GetRootComponent` _actorlanzado)))
    (`PrimitiveComponent.IgnoreActorWhenMoving` _asprimitive_component (`self.GetOwner`) false)))