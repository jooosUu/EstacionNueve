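; Detector component that computes the owning character's noise level and handles an upgradeable sensor scan.
; A looping timer combines movement state, carried Comprimidos and temporary one-off noise, scales it by the traced surface's physical material, subtracts ambient noise and reports to the GameInstance.
; Scanning messages BPI_Interactuable actors in a sphere, with higher levels reaching farther more quietly; its cooldown check only proceeds when the flag is already set.
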(event `self.ReceiveBeginPlay`
  (set `self.Inventario` (`Actor.GetComponentByClass` (`self.GetOwner`) "/Game/EstacionNueve/Componentes/AC_Inventario.AC_Inventario_C"))
  (`KismetSystemLibrary.K2_SetTimer` self "ActualizarRuido" 0.2 true))

(fn `ActualizarRuido`
  (locals (Velocidad :type "Float (single-precision)" :default 0.0) (dBBase :type "Float (single-precision)" :default 0.0) (ExtraRuido :type "Float (single-precision)" :default 0.0) (DbMovimiento :type "Float (single-precision)") (DbTotal :type "Float (single-precision)") (Multiplicador :type "Float (single-precision)") (NombrePM :type Name) (bCaminando :type Boolean))
  (bind _returnvalue (`self.GetOwner`))
  (bind _velocidadcorrerminima (`self.VelocidadCorrerMinima`))
  (bind _velocidadquietomaxima (`self.VelocidadQuietoMaxima`))
  (bind _inventario (`self.Inventario`))
  (bind _dbtotal (`local.DbTotal`))
  (bind _returnvalue_2 (`Actor.K2_GetActorLocation` _returnvalue))
  (bind (_value _returnvalue_3) (`BlueprintMapLibrary.Map_Find` (`self.MultiplicadoresSuperficie`) (`local.NombrePM`)))
  (bind _returnvalue_4 (`KismetMathLibrary.VSize` (`Actor.GetVelocity` _returnvalue)))
  (bind _returnvalue_5 (`NavMovementComponent.IsCrouching` (`Actor.GetComponentByClass` _returnvalue "/Script/Engine.CharacterMovementComponent")))
  (bind _returnvalue_6 (and (not _returnvalue_5) (and (<= _returnvalue_4 _velocidadcorrerminima) (>= _returnvalue_4 _velocidadquietomaxima))))
  (set `local.Velocidad` _returnvalue_4)
  (set `local.DbMovimiento` (+ (`KismetMathLibrary.SelectFloat` (`self.DbAgachado`) (`KismetMathLibrary.SelectFloat` (`self.DbCorrer`) (`KismetMathLibrary.SelectFloat` (`self.DbQuieto`) (`self.DbCaminar`) (< _returnvalue_4 _velocidadquietomaxima)) (> _returnvalue_4 _velocidadcorrerminima)) _returnvalue_5) (`KismetMathLibrary.SelectFloat` (`self.DbExtraPorComprimido`) 0.0 (and _returnvalue_6 (and (`KismetSystemLibrary.IsValid` _inventario) (>= (`/Game/EstacionNueve/Componentes/AC_Inventario.GetNumComprimidos` _inventario) 1))))))
  (set `local.bCaminando` _returnvalue_6)
  (bind _outhit (`KismetSystemLibrary.LineTraceSingle` _returnvalue_2 (- _returnvalue_2 (`KismetMathLibrary.MakeVector` 0.0 0.0 (`self.DistanciaTraceSuperficie`))) "TraceTypeQuery1"))
  (set `local.NombrePM` (`KismetStringLibrary.Conv_StringToName` (`KismetSystemLibrary.GetObjectName` (`.PhysMat` (`GameplayStatics.BreakHitResult` _outhit)))))
  (set `local.Multiplicador` (`KismetMathLibrary.SelectFloat` _value (`self.MultiplicadorSuperficiePorDefecto`) _returnvalue_3))
  (set `local.DbTotal` (+ (`local.DbMovimiento`) (`self.DbPuntual`)))
  (set `local.DbTotal` (* _dbtotal (`local.Multiplicador`)))
  (bind _asbp_gi_estacion_nueve (cast `/Game/EstacionNueve/Core/BP_GI_EstacionNueve` (`GameplayStatics.GetGameInstance`))
    (:`then`
      (set `local.DbTotal` (`KismetMathLibrary.FMax` (- _dbtotal (`/Game/EstacionNueve/Core/BP_GI_EstacionNueve.RuidoAmbientalDb` _asbp_gi_estacion_nueve))))
      (set `self.CurrentNoise_dB` _dbtotal)
      (`self.OnRuidoCambiado` _dbtotal)
      (if (> _dbtotal 0.0)
        (`/Game/EstacionNueve/Core/BP_GI_EstacionNueve.ReportNoise` _asbp_gi_estacion_nueve _returnvalue_2 _dbtotal "NewEnumerator0" _returnvalue)))
    (:`CastFailed`
      (set `self.CurrentNoise_dB` _dbtotal)
      (`self.OnRuidoCambiado` _dbtotal))))

(fn `Escanear`
  (locals (Radio :type "Float (single-precision)" :default 0.0) (RuidoEscaneo :type "Float (single-precision)" :default 0.0) (ActoresCercanos :type "Array of Actor Object Reference"))
  (bind _returnvalue (`self.GetOwner`))
  (bind _sensorlevel (`self.SensorLevel`))
  (bind _returnvalue_2 (`Actor.K2_GetActorLocation` _returnvalue))
  (if (`self.bSensorInstalado`)
    (if (`self.bEscaneoEnEnfriamiento`)
      (set `self.bEscaneoEnEnfriamiento` true)
      (`KismetSystemLibrary.K2_SetTimer` self "FinEscaneoEnfriamiento" 3.0)
      (if (== _sensorlevel 1)
        (set `local.Radio` 600.0)
        (set `local.RuidoEscaneo` 30.0)
        (elif (== _sensorlevel 2)
          (set `local.Radio` 1200.0)
          (set `local.RuidoEscaneo` 22.0)
          (else
            (set `local.Radio` 2000.0)
            (set `local.RuidoEscaneo` 10.0))))
      (bind _outactors (`KismetSystemLibrary.SphereOverlapActors` _returnvalue_2 (`local.Radio`) (`|MakeArray` "ObjectTypeQuery2" "ObjectTypeQuery3" "ObjectTypeQuery1" :!type "EObjectTypeQuery Enum") "/Script/Engine.Actor"))
      (for _array_element _outactors
        (if (`KismetSystemLibrary.DoesImplementInterface` _array_element "/Game/EstacionNueve/Core/BPI_Interactuable.BPI_Interactuable_C")
          (message `/Game/EstacionNueve/Core/BPI_Interactuable.E_OnScanned` _array_element (`self.SensorLevel`))))
      (bind _asbp_gi_estacion_nueve (cast `/Game/EstacionNueve/Core/BP_GI_EstacionNueve` (`GameplayStatics.GetGameInstance`)))
      (`/Game/EstacionNueve/Core/BP_GI_EstacionNueve.ReportNoise` _asbp_gi_estacion_nueve _returnvalue_2 (`local.RuidoEscaneo`) "NewEnumerator3" _returnvalue)
      (`self.OnEscaneoRealizado` (`self.SensorLevel`)))))

(fn `FinEscaneoEnfriamiento`
  (set `self.bEscaneoEnEnfriamiento` false))

(fn `InstalarSensor`
  (set `self.bSensorInstalado` true)
  (`self.OnSensorMejorado` 1))

(fn `LimpiarPuntual`
  (set `self.DbPuntual` 0.0))

(fn `MejorarSensor`
  (set `self.SensorLevel` (`KismetMathLibrary.Min` (+ (`self.SensorLevel`) 1) 3))
  (`self.OnSensorMejorado` (`self.SensorLevel`)))

(fn `ReportarRuidoPuntual`
  (params (dB :type "Float (single-precision)") (Fuente :type "/Game/EstacionNueve/Core/E_NoiseSource Enum" :default "NewEnumerator0"))
  (set `self.DbPuntual` dB)
  (`KismetSystemLibrary.K2_ClearAndInvalidateTimerHandle` (`self.TimerPuntual`))
  (bind _returnvalue (`KismetSystemLibrary.K2_SetTimer` self "LimpiarPuntual" (`self.DuracionPuntual`)))
  (set `self.TimerPuntual` _returnvalue))