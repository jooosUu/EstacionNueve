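; BP_Herramienta_Pico is a pickaxe tool that strikes what its owner is looking at and makes noise.
; On a hit event, Golpear line-traces from the owner's camera and applies point damage to whatever it hits.
; Each swing also reports a noise burst to the owner's AC_Detector, cached on BeginPlay, even if it misses.
; A timer-driven cooldown gates repeated swings.
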(event `self.ReceiveBeginPlay`
  (`|ExecutionSequence`
    (:`then_0`
      (bind _asac_detector (cast `/Game/EstacionNueve/Componentes/AC_Detector` (`self.GetComponentByClass` (`self.GetOwner` self) "/Game/EstacionNueve/Componentes/AC_Detector.AC_Detector_C")))
      (set `self.Detector` _asac_detector))))

(event `FinCooldown`
  (set `self.bPuedeGolpear` true))

(event `self.E_Hit`
  (`self.Golpear`))

(fn `GetInteractionPrompt`
  (returns (Prompt :type Text))
  (return ""))

(fn `Golpear`
  (bind _detector (`self.Detector`))
  (bind _returnvalue (`self.GetOwner` self))
  (if (`self.bPuedeGolpear`)
    (set `self.bPuedeGolpear` false)
    (`KismetSystemLibrary.K2_SetTimer` self "FinCooldown" (`self.Cadencia`))
    (bind _ascamera_component (cast `CameraComponent` (`self.GetComponentByClass` _returnvalue "/Script/Engine.CameraComponent")))
    (`|ExecutionSequence`
      (:`then_0`
        (bind _returnvalue_2 (`SceneComponent.K2_GetComponentLocation` _ascamera_component))
        (bind _returnvalue_3 (`SceneComponent.GetForwardVector` _ascamera_component))
        (bind (_outhit _returnvalue_4) (`KismetSystemLibrary.LineTraceSingle` _returnvalue_2 (+ _returnvalue_2 (* _returnvalue_3 (`self.Alcance`))) "TraceTypeQuery1"))
        (`/Engine/EditorBlueprintResources/StandardMacros.IsValid` _detector
          (:`Is Valid`
            (`/Game/EstacionNueve/Componentes/AC_Detector.ReportarRuidoPuntual` _detector (`self.Ruido_dB`) "NewEnumerator1"))))
      (:`then_1`
        (if _returnvalue_4
          (`GameplayStatics.ApplyPointDamage` (`.HitActor` (`GameplayStatics.BreakHitResult` _outhit)) (`self.Dano`) _returnvalue_3 _outhit (`self.GetInstigatorController` _returnvalue) self (`self.TipoDano`)))))))

(fn `UserConstructionScript`)