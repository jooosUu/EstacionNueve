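; BP_Arma_Base is a base weapon that handles hitscan firing, ammo, reloading and equip visibility.
; Disparar traces one or more pellets in a random cone from the owner's camera, applying point damage, doubled on headshots, with a timer limiting fire rate.
; Each shot reports noise to the owner's AC_Detector.
; Recargar moves rounds one at a time from AC_Inventario on a timer, blocking fire meanwhile, and ammo changes are broadcast.
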(event `self.ReceiveBeginPlay`
  (set `self.Inventario` (`self.GetComponentByClass` (`self.GetOwner` self) "/Game/EstacionNueve/Componentes/AC_Inventario.AC_Inventario_C"))
  (set `self.Detector` (`self.GetComponentByClass` (`self.GetOwner` self) "/Game/EstacionNueve/Componentes/AC_Detector.AC_Detector_C"))
  (set `self.bPuedeDisparar` true))

(event `self.ReceiveActorBeginOverlap`
  (params (OtherActor :type "Actor Object Reference")))

(event `self.ReceiveTick`
  (params (DeltaSeconds :type "Float (single-precision)")))

(event `self.E_Fire`
  (`self.Disparar`))

(event `self.E_Reload`
  (`self.Recargar`))

(fn `Desequipar`
  (`SceneComponent.SetVisibility` (`self.Malla`) false false)
  (set `self.bPuedeDisparar` false))

(fn `Disparar`
  (locals (DanoFinal :type "Float (single-precision)" :default 0.0) (InicioRayo :type "Vector Structure") (DireccionDisparo :type "Vector Structure") (FinRayo :type "Vector Structure"))
  (bind _iniciorayo (`local.InicioRayo`))
  (bind _dano (`self.Dano`))
  (bind _returnvalue (`self.GetOwner` self))
  (bind _returnvalue_2 (`self.GetComponentByClass` _returnvalue "/Script/Engine.CameraComponent"))
  (bind _returnvalue_3 (`KismetMathLibrary.RandomUnitVectorInConeInDegrees` (`KismetMathLibrary.GetForwardVector` (`SceneComponent.K2_GetComponentRotation` _returnvalue_2)) (`self.DispersionGrados`)))
  (bind _returnvalue_4 (+ _iniciorayo (* _returnvalue_3 (`self.Alcance`))))
  (if (`self.bPuedeDisparar`)
    (if (not (`self.bRecargando`))
      (if (> (`self.EnCargador`) 0)
        (set `self.bPuedeDisparar` false)
        (`KismetSystemLibrary.K2_SetTimer` self "FinCadencia" (`self.Cadencia`))
        (set `local.InicioRayo` (`SceneComponent.K2_GetComponentLocation` _returnvalue_2))
        (for _ (range (`self.Perdigones`))
          (set `local.DireccionDisparo` _returnvalue_3)
          (set `local.FinRayo` _returnvalue_4)
          (bind (_outhit _returnvalue_5) (`KismetSystemLibrary.LineTraceSingle` _iniciorayo _returnvalue_4 "TraceTypeQuery1"))
          (if _returnvalue_5
            (`|ExecutionSequence`
              (:`then_0`
                (set `local.DanoFinal` _dano)
                (bind (_bblockinghit _binitialoverlap _time _distance _location _impactpoint _normal _impactnormal _physmat _hitactor _hitcomponent _hitbonename _bonename) (`GameplayStatics.BreakHitResult` _outhit))
                (if (or (== _bonename "head") (`ActorComponent.ComponentHasTag` _hitcomponent "Cabeza"))
                  (set `local.DanoFinal` (* _dano 2.0))))
              (:`then_1`
                (`GameplayStatics.ApplyPointDamage` _hitactor (`local.DanoFinal`) _returnvalue_3 _outhit (`Pawn.GetController` (`self.GetInstigator` _returnvalue)) self (`self.TipoDano`))))))
        (set `self.EnCargador` (- (`self.EnCargador`) 1))
        (`/Game/EstacionNueve/Componentes/AC_Detector.ReportarRuidoPuntual` (`self.Detector`) (`self.Ruido_dB`) "NewEnumerator2")
        (`self.OnMunicionCambiada` (`self.EnCargador`) (`/Game/EstacionNueve/Componentes/AC_Inventario.GetCantidad` (`self.Inventario`) (`self.MunicionID`)))))))

(fn `Equipar`
  (`SceneComponent.SetVisibility` (`self.Malla`) true false)
  (`self.SetActorHiddenInGame` self false)
  (set `self.bPuedeDisparar` true))

(fn `FinCadencia`
  (set `self.bPuedeDisparar` true))

(fn `GetInteractionPrompt`
  (returns (Prompt :type Text))
  (return ""))

(fn `Recargar`
  (if (`self.bRecargando`)
    _
    (elif (not (>= (`self.EnCargador`) (`self.Capacidad`)))
      (set `self.bRecargando` true)
      (`self.RecargarUnaBala`))))

(fn `RecargarUnaBala`
  (bind _municionid (`self.MunicionID`))
  (bind _inventario (`self.Inventario`))
  (if (or (>= (`self.EnCargador`) (`self.Capacidad`)) (<= (`/Game/EstacionNueve/Componentes/AC_Inventario.GetCantidad` _inventario _municionid) 0))
    (set `self.bRecargando` false)
    (else
      (bind _bexito (`/Game/EstacionNueve/Componentes/AC_Inventario.Quitar` _inventario _municionid 1))
      (if _bexito
        (set `self.EnCargador` (+ (`self.EnCargador`) 1))
        (`self.OnMunicionCambiada` (`self.EnCargador`) (`/Game/EstacionNueve/Componentes/AC_Inventario.GetCantidad` (`self.Inventario`) (`self.MunicionID`)))
        (`KismetSystemLibrary.K2_SetTimer` self "RecargarUnaBala" (`self.TiempoRecargaPorBala`))
        (else
          (set `self.bRecargando` false))))))

(fn `UserConstructionScript`)