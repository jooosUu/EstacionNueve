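; AI controller for the Carnotaurus, a sound-driven predator that wanders, investigates, hunts or gets stunned.
; Noise events bound from the game instance are weighed by loudness and distance: moderate ones draw investigation, louder ones start a hunt on the instigator, very loud close ones stun it.
; Looping timers, rather than Tick or a behavior tree, drive navmesh movement, with speed set per state.
; Hunts end at long range or trigger cooldown-gated bites up close.
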(event `self.ReceiveBeginPlay`
  (set `self.Estado` "Deambular")
  (`self.IniciarDeambular`)
  (bind _asbp_gi_estacion_nueve (cast `/Game/EstacionNueve/Core/BP_GI_EstacionNueve` (`GameplayStatics.GetGameInstance`)))
  (add `/Game/EstacionNueve/Core/BP_GI_EstacionNueve.OnNoise` _asbp_gi_estacion_nueve (`|CreateDelegate` :!event `AlOirRuido`)))

(event `self.ReceiveTick`
  (params (DeltaSeconds :type "Float (single-precision)")))

(event `AlOirRuido`
  (params (Location :type "Vector Structure") (dB :type "Float (double-precision)") (Fuente :type "/Game/EstacionNueve/Core/E_NoiseSource Enum" :default "NewEnumerator0") (Instigador :type "Actor Object Reference"))
  (bind _returnvalue (`KismetMathLibrary.VSize` (- Location (`self.K2_GetActorLocation` (`self.K2_GetPawn`)))))
  (if (== (`self.Estado`) "Aturdido")
    _
    (elif (and (>= dB (`self.UmbralAturdir`)) (<= _returnvalue (`self.RadioAturdir`)))
      (set `self.Estado` "Aturdido")
      (`self.StopMovement`)
      (`KismetSystemLibrary.K2_ClearAndInvalidateTimerHandle` (`self.TimerCazar`))
      (bind _ascharacter (cast `Character` (`self.K2_GetPawn`))
        (:`then`
          (`Character.PlayAnimMontage` _ascharacter "/Game/EstacionNueve/IA/AM_Carno_Dano.AM_Carno_Dano" 1.0 "None"))
        (:`CastFailed`
          _))
      (`KismetSystemLibrary.Delay` (`self.DuracionAturdido`))
      (if (== (`self.Estado`) "Aturdido")
        (set `self.Estado` "Deambular"))
      (elif (<= _returnvalue (* dB (`self.RadioPorDb`)))
        (if (> dB (`self.UmbralCaza`))
          (set `self.ObjetivoJugador` Instigador)
          (set `self.Estado` "Cazar")
          (`self.IniciarCaza`)
          (elif (`KismetStringLibrary.NotEqual_StrStr` (`KismetStringLibrary.Conv_NameToString` (`self.Estado`)) "Cazar")
            (if (> dB (`self.UmbralInvestigar`))
              (set `self.UltimoRuidoLoc` Location)
              (set `self.Estado` "Investigar")
              (`self.InvestigarRuido`))))))))

(event `ActualizarCaza`
  (bind (_projectedlocation _returnvalue) (`NavigationSystemV1.K2_ProjectPointToNavigation` (`self.DestinoActual`) null null (`KismetMathLibrary.MakeVector` 200.0 200.0 500.0)))
  (`|ExecutionSequence`
    (:`then_0`
      (if (not (`KismetSystemLibrary.IsValid` (`self.ObjetivoJugador`)))
        (`KismetSystemLibrary.K2_ClearAndInvalidateTimerHandle` (`self.TimerCazar`))
        (set `self.Estado` "Deambular")
        (elif (`|EnumInequality` (`self.GetMoveStatus`) "Moving")
          (set `self.DestinoActual` (`self.K2_GetActorLocation` (`self.ObjetivoJugador`)))
          (if _returnvalue
            (bind _returnvalue_2 (`self.MoveToLocation` self _projectedlocation 250.0 false true false true null true))
            (set `self.bMovimientoIniciado` (`|EnumEquality` _returnvalue_2 "RequestSuccessful"))
            (else
              (set `self.bMovimientoIniciado` false))))))
    (:`then_1`
      (if (> (`self.GetDistanceTo` (`self.K2_GetPawn`) (`self.ObjetivoJugador`)) 3000.0)
        (`KismetSystemLibrary.K2_ClearAndInvalidateTimerHandle` (`self.TimerCazar`))
        (set `self.Estado` "Deambular")))
    (:`then_2`
      (if (<= (`self.GetDistanceTo` (`self.K2_GetPawn`) (`self.ObjetivoJugador`)) (`self.RangoAtaque`))
        (`self.EjecutarAtaque`)))))

(fn `ActualizarVelocidad`)

(fn `EjecutarAtaque`
  (bind _returnvalue (`self.K2_GetPawn` self))
  (if (not (`self.bEstaAtacando`))
    (set `self.bEstaAtacando` true)
    (bind _ascharacter (cast `Character` _returnvalue))
    (`Character.PlayAnimMontage` _ascharacter "/Game/EstacionNueve/IA/AM_Carno_Ataque.AM_Carno_Ataque" 1.0 "None")
    (`GameplayStatics.ApplyDamage` (`self.ObjetivoJugador`) 25.0 self _returnvalue "/Game/EstacionNueve/Core/DT_Mordisco.DT_Mordisco_C")
    (`KismetSystemLibrary.K2_SetTimerDelegate` (`|CreateDelegate` :!event `TerminarAtaque`) 1.5)))

(fn `EjecutarDeambular`
  (bind _estado (`self.Estado`))
  (bind _returnvalue (`self.K2_GetPawn` self))
  (bind (_randomlocation _returnvalue_2) (`NavigationSystemV1.K2_GetRandomReachablePointInRadius` self (`self.K2_GetActorLocation` _returnvalue) 1500.0 null null))
  (bind _ascharacter (cast `Character` _returnvalue))
  (if (== _estado "Deambular")
    (set `CharacterMovementComponent.MaxWalkSpeed` 200.0 (`Character.CharacterMovement` _ascharacter))
    (if (and (< (`KismetMathLibrary.VSize` (`self.GetVelocity` _returnvalue)) 20.0) _returnvalue_2)
      (if (`KismetMathLibrary.RandomBoolWithWeight` 0.0)
        (`Character.PlayAnimMontage` _ascharacter "/Game/EstacionNueve/IA/AM_Carno_Alerta.AM_Carno_Alerta" 1.0 "None")
        (else
          (`self.MoveToLocation` self _randomlocation 100.0 true true false true null true))))
    (elif (== _estado "Investigar")
      (if (<= (`KismetMathLibrary.VSize` (- (`self.UltimoRuidoLoc`) (`self.K2_GetActorLocation` _returnvalue))) 300.0)
        (set `self.Estado` "Deambular")))))

(fn `IniciarCaza`
  (bind _ascharacter (cast `Character` (`self.K2_GetPawn`)))
  (set `CharacterMovementComponent.MaxWalkSpeed` 600.0 (`Character.CharacterMovement` _ascharacter))
  (`KismetSystemLibrary.K2_ClearAndInvalidateTimerHandle` (`self.TimerCazar`))
  (bind _returnvalue (`KismetSystemLibrary.K2_SetTimerDelegate` (`|CreateDelegate` :!event `ActualizarCaza`) 0.3 true))
  (set `self.TimerCazar` _returnvalue))

(fn `IniciarDeambular`
  (bind _returnvalue (`KismetSystemLibrary.K2_SetTimerDelegate` (`|CreateDelegate` :!event `EjecutarDeambular`) 4.0 true))
  (set `self.TimerDeambular` _returnvalue))

(fn `InvestigarRuido`
  (bind _ultimoruidoloc (`self.UltimoRuidoLoc`))
  (bind (_projectedlocation _returnvalue) (`NavigationSystemV1.K2_ProjectPointToNavigation` _ultimoruidoloc null null (`KismetMathLibrary.MakeVector` 200.0 200.0 500.0)))
  (bind _ascharacter (cast `Character` (`self.K2_GetPawn`)))
  (`|ExecutionSequence`
    (:`then_0`
      (set `CharacterMovementComponent.MaxWalkSpeed` 350.0 (`Character.CharacterMovement` _ascharacter))
      (set `self.DestinoActual` _ultimoruidoloc)
      (if _returnvalue
        (bind _returnvalue_2 (`self.MoveToLocation` self _projectedlocation 150.0 false true false true null true))
        (set `self.bMovimientoIniciado` (`|EnumEquality` _returnvalue_2 "RequestSuccessful"))
        (else
          (set `self.bMovimientoIniciado` false))))
    (:`then_1`
      (set `self.Estado` "Investigar"))))

(fn `OnRuidoEscuchado`)

(fn `TerminarAtaque`
  (set `self.bEstaAtacando` false))

(fn `UserConstructionScript`)