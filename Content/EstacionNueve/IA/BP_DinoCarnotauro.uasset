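; BP_DinoCarnotauro is an AI-controlled Carnotaurus that the player can mount and ride.
; Montar attaches the player character without collision, damage or movement tick, then swaps possession from the stored AI controller to the player.
; While mounted, it handles camera-relative movement, sprint and a V toggle between two cameras, hiding the rider when CamaraJinete is active.
; IA_Interact drops the rider to the side and returns both pawns to their controllers.
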(event `self.ReceiveBeginPlay`
  (set `CharacterMovementComponent.bOrientRotationToMovement` true (`self.CharacterMovement`)))

(event `EnhancedInput|/Game/Input/Actions/IA_Interact`
  (params (ActionValue :type Boolean) (ElapsedSeconds :type "Float (double-precision)") (TriggeredSeconds :type "Float (double-precision)") (InputAction :type "InputAction Object Reference" :default "/Game/Input/Actions/IA_Interact.IA_Interact"))
  (bind _returnvalue (`GameplayStatics.GetPlayerController` 0))
  (bind _jinete (`self.Jinete`))
  (:`Started`
    (if (`self.bMontado`)
      (set `self.bMontado` false)
      (`self.K2_DetachFromActor` _jinete "KeepWorld" "KeepWorld" "KeepWorld")
      (`self.SetActorHiddenInGame` (`self.Jinete`) false)
      (`self.K2_SetActorLocation` _jinete (+ (`self.K2_GetActorLocation`) (* (`self.GetActorRightVector`) (330.0 330.0 330.0))) false true)
      (`self.SetActorEnableCollision` _jinete true)
      (`ActorComponent.SetComponentTickEnabled` (`self.GetMovementComponent` _jinete) true)
      (set `Actor.bCanBeDamaged` true _jinete)
      (`Controller.Possess` (`self.ControladorIA`) (`Controller.K2_GetPawn` _returnvalue))
      (`Controller.Possess` _returnvalue _jinete))))

(event `Montar`
  (bind _jinete (`self.Jinete`))
  (set `self.Jinete` (`GameplayStatics.GetPlayerCharacter` 0))
  (set `self.ControladorIA` (`self.GetController`))
  (set `self.bMontado` true)
  (`self.SetActorEnableCollision` _jinete false)
  (`ActorComponent.SetComponentTickEnabled` (`self.GetMovementComponent` _jinete) false)
  (set `Actor.bCanBeDamaged` false _jinete)
  (`self.K2_AttachToComponent` _jinete (`self.CapsuleComponent`) "None" "SnapToTarget" "SnapToTarget" "KeepWorld" true)
  (`self.K2_SetActorRelativeLocation` _jinete (0.0 0.0 140.0) false false)
  (`self.SetActorHiddenInGame` (`self.Jinete`) (`ActorComponent.IsActive` (`self.CamaraJinete`)))
  (`Controller.Possess` (`GameplayStatics.GetPlayerController` 0) (`Controller.K2_GetPawn` (`self.ControladorIA`)))
  (set `CharacterMovementComponent.MaxWalkSpeed` 350.0 (`self.CharacterMovement`)))

(event `EnhancedInput|/Game/Input/Actions/IA_Move`
  (params (ActionValue :type "Vector2D Structure") (ElapsedSeconds :type "Float (double-precision)") (TriggeredSeconds :type "Float (double-precision)") (InputAction :type "InputAction Object Reference" :default "/Game/Input/Actions/IA_Move.IA_Move"))
  (bind (_x _y) (`KismetMathLibrary.BreakVector2D` ActionValue))
  (bind _returnvalue (`KismetMathLibrary.MakeRotator` 0.0 0.0 (.yaw (`self.GetControlRotation`))))
  (:`Triggered`
    (if (`self.bMontado`)
      (`self.AddMovementInput` (`KismetMathLibrary.GetForwardVector` _returnvalue) _y)
      (`self.AddMovementInput` (`KismetMathLibrary.GetRightVector` _returnvalue) _x))))

(event `EnhancedInput|/Game/Input/Actions/IA_Look`
  (params (ActionValue :type "Vector2D Structure") (ElapsedSeconds :type "Float (double-precision)") (TriggeredSeconds :type "Float (double-precision)") (InputAction :type "InputAction Object Reference" :default "/Game/Input/Actions/IA_Look.IA_Look"))
  (bind (_x _y) (`KismetMathLibrary.BreakVector2D` ActionValue))
  (:`Triggered`
    (`self.AddControllerYawInput` _x)
    (`self.AddControllerPitchInput` (* _y -1.0))))

(event `EnhancedInput|/Game/Input/Actions/IA_Sprint`
  (params (ActionValue :type Boolean) (ElapsedSeconds :type "Float (double-precision)") (TriggeredSeconds :type "Float (double-precision)") (InputAction :type "InputAction Object Reference" :default "/Game/Input/Actions/IA_Sprint.IA_Sprint"))
  (:`Started`
    (if (`self.bMontado`)
      (set `CharacterMovementComponent.MaxWalkSpeed` 600.0 (`self.CharacterMovement`))))
  (:`Completed`
    (if (`self.bMontado`)
      (set `CharacterMovementComponent.MaxWalkSpeed` 350.0 (`self.CharacterMovement`)))))

(event `Key|V`
  (params (Key :type "Key Structure"))
  (:`Pressed`
    (if (`self.bMontado`)
      (`ActorComponent.ToggleActive` (`self.CamaraMontura`))
      (`ActorComponent.ToggleActive` (`self.CamaraJinete`))
      (`self.SetActorHiddenInGame` (`self.Jinete`) (`ActorComponent.IsActive` (`self.CamaraJinete`))))))

(fn `UserConstructionScript`)