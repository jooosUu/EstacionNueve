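; Explosive barrel actor that blows up when it takes any damage or when E is pressed with the player within range.
; Both triggers call Explotar, which applies radial damage, fires a radial force impulse, shows debug sphere and message, then destroys the actor.
; It enables player input on itself at BeginPlay for the key.
; The Explotado guard sets the flag to false, so it never blocks re-entry.
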(event `Explotar`
  (bind _returnvalue (`self.K2_GetActorLocation`))
  (if (not (`self.bExplotado`))
    (set `self.bExplotado` false)
    (`GameplayStatics.ApplyRadialDamage` :`BaseDamage` 100.0 :`Origin` _returnvalue :`DamageRadius` 650.0 :`DamageCauser` null :`InstigatedByController` null)
    (`RadialForceComponent.FireImpulse` (`self.FuerzaRadial`))
    (`KismetSystemLibrary.DrawDebugSphere` _returnvalue 650.0 16 (struct :`R` 1.0 :`G` 0.25 :`B` 0.05 :`A` 1.0) 2.0 4.0)
    (`KismetSystemLibrary.PrintString` "¡BOOM! El barril exploto e infligio 100 de dano radial en un radio de 650 cm." true true (struct :`R` 1.0 :`G` 0.3 :`B` 0.1 :`A` 1.0) 4.0)
    (`self.K2_DestroyActor`)))

(event `self.ReceiveBeginPlay`
  (`self.EnableInput` (`GameplayStatics.GetPlayerController` 0)))

(event `self.ReceiveAnyDamage`
  (params (Damage :type "Float (single-precision)") (DamageType :type "DamageType Object Reference") (InstigatedBy :type "Controller Object Reference") (DamageCauser :type "Actor Object Reference"))
  (`self.Explotar`))

(event `Key|E`
  (params (Key :type "Key Structure"))
  (:`Pressed`
    (if (<= (`KismetMathLibrary.Vector_Distance` (`self.K2_GetActorLocation` (`GameplayStatics.GetPlayerCharacter` 0)) (`self.K2_GetActorLocation`)) 450.0)
      (`self.Explotar`))))

(fn `UserConstructionScript`)