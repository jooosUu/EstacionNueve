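; BP_Door is an interactable hinged door that the player opens and closes with E when nearby.
; Tick polls the key and distance, then eases the Hinge yaw toward open or closed with FInterpTo.
; If NeedsKey is set, it stays locked with a printed message while any BP_KeyPickup actor still exists in the level.
; ToggleDoor flips the door and plays its sound directly, skipping those checks.
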(event `self.ReceiveTick`
  (params (DeltaSeconds :type "Float (single-precision)"))
  (bind _bopen (`self.bOpen`))
  (bind _returnvalue (`KismetMathLibrary.FInterpTo` (`self.CurrentYaw`) (`KismetMathLibrary.SelectFloat` -90.0 0.0 _bopen) DeltaSeconds 5.0))
  (`|ExecutionSequence`
    (:`then_0`
      (if (and (`PlayerController.WasInputKeyJustPressed` (`GameplayStatics.GetPlayerController` 0) "E") (`KismetMathLibrary.InRange_FloatFloat` (`KismetMathLibrary.Vector_Distance` (`self.K2_GetActorLocation` (`GameplayStatics.GetPlayerPawn` 0)) (`self.K2_GetActorLocation`)) 0.0 300.0))
        (if (`self.bNeedsKey`)
          (bind _returnvalue_2 (`GameplayStatics.GetActorOfClass` "/Game/Blueprints/BP_KeyPickup.BP_KeyPickup_C"))
          (if (`KismetSystemLibrary.IsValid` _returnvalue_2)
            (`KismetSystemLibrary.PrintString` "Puerta cerrada con llave! Recoge primero la Llave Dorada [E]." true true (struct :`G` 0.66 :`B` 1.0 :`A` 1.0) 3.5)
            (else
              (set `self.bOpen` (not _bopen) :!label _label)
              (`GameplayStatics.PlaySound2D` "/Engine/VREditor/Sounds/UI/Dockable_Window_Open.Dockable_Window_Open" 1.0 1.0 0.0 null null)))
          (else
            (goto _label)))))
    (:`then_1`
      (set `self.CurrentYaw` _returnvalue)
      (`SceneComponent.K2_SetRelativeRotation` (`self.Hinge`) (`KismetMathLibrary.MakeRotator` 0.0 0.0 _returnvalue) false false))))

(event `ToggleDoor`
  (goto _label))

(fn `UserConstructionScript`)