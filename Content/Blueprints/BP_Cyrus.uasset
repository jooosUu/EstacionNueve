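; BP_Cyrus is a playable character Blueprint with sprint, crouch and hitscan shooting, all bound directly to keyboard and mouse keys.
; Left Shift switches walk speed, while Left Ctrl toggles crouch and also squashes the actor's vertical scale.
; Left click traces the Visibility channel along the actor's forward vector rather than a camera, damaging any hit actor and printing a Spanish confirmation message.
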(event `Key|LeftShift`
  (params (Key :type "Key Structure"))
  (bind _charactermovement (`self.CharacterMovement`))
  (:`Pressed`
    (set `CharacterMovementComponent.MaxWalkSpeed` 600.0 _charactermovement))
  (:`Released`
    (set `CharacterMovementComponent.MaxWalkSpeed` 350.0 _charactermovement)))

(event `Key|LeftControl`
  (params (Key :type "Key Structure"))
  (:`Pressed`
    (`self.Crouch`)
    (`self.SetActorScale3D` (1.0 1.0 0.55)))
  (:`Released`
    (`self.UnCrouch`)
    (`self.SetActorScale3D` (1.0 1.0 1.0))))

(event `Key|LeftMouseButton`
  (params (Key :type "Key Structure"))
  (bind _returnvalue (`self.K2_GetActorLocation`))
  (:`Pressed`
    (bind (_outhit _returnvalue_2) (`KismetSystemLibrary.LineTraceSingle` _returnvalue (+ _returnvalue (* (`self.GetActorForwardVector`) 3000.0)) "TraceTypeQuery1"))
    (if _returnvalue_2
      (`GameplayStatics.ApplyDamage` (`.HitActor` (`GameplayStatics.BreakHitResult` _outhit)) 100.0)
      (`KismetSystemLibrary.PrintString` "¡Disparo! Daño aplicado al objetivo." true true (struct :`G` 0.66 :`B` 1.0 :`A` 1.0) 3.0))))

(fn `UserConstructionScript`
  (`parent.UserConstructionScript`))