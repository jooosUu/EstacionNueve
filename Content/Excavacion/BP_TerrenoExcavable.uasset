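; Diggable rock terrain on a dynamic mesh, with a seeded procedurally generated cave and mineral veins.
; On BeginPlay, GenerarCaverna subtracts a random-walk tunnel of unioned spheres from a box using Geometry Script booleans.
; After a delay, traces from tunnel points place veins on the walls, some with dinosaur amber buried behind them below actor height.
; Excavar subtracts a Perlin-noised sphere at the dig point and refreshes complex collision.
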(event `self.ReceiveBeginPlay`
  (`PrimitiveComponent.SetMaterial` (`self.GetDynamicMeshComponent`) 0 "/Game/Excavacion/Materiales/M_Roca.M_Roca")
  (`self.GenerarCaverna`))

(event `GenerarCaverna`
  (bind _mallaherramienta (`self.MallaHerramienta`))
  (bind _stream (`self.Stream`))
  (bind _clasesveta (`self.ClasesVeta`))
  (bind _x (.x (`self.Tamano`)))
  (bind _z (.z (`self.Tamano`)))
  (bind _returnvalue (* (.y (`self.Tamano`)) 0.5))
  (bind _returnvalue_2 (* (.z (`self.Tamano`)) 0.5))
  (bind _returnvalue_3 (- (* _x -0.5) 200.0))
  (`KismetArrayLibrary.Array_Clear` (`self.PuntosTunel`))
  (set `self.Stream` (`KismetMathLibrary.MakeRandomStream` (`self.Semilla`)))
  (bind _returnvalue_4 (`BaseDynamicMeshComponent.GetDynamicMesh` (`self.GetDynamicMeshComponent`)))
  (bind _returnvalue_5 (`DynamicMesh.Reset` _returnvalue_4))
  (`GeometryScriptLibrary_MeshPrimitiveFunctions.AppendBox` _returnvalue_5 (struct) (struct) _x (.y (`self.Tamano`)) _z 8 6 4 "Center")
  (bind _returnvalue_6 (`self.AllocateComputeMesh`))
  (set `self.MallaHerramienta` _returnvalue_6)
  (set `self.Pos` (`KismetMathLibrary.MakeVector` _returnvalue_3 0.0 (- (* _z 0.5) 650.0)))
  (set `self.Dir` (1.0 0.0 -0.15))
  (for _ (range (`self.PasosTunel`))
    (bind _output_get (set `self.Dir` (`KismetMathLibrary.Normal` (+ (+ (`self.Dir`) (* (`KismetMathLibrary.RandomUnitVectorFromStream` (`self.Stream`)) 0.35)) (0.4 0.0 -0.05)))))
    (bind _output_get_2 (set `self.Pos` (`KismetMathLibrary.MakeVector` (`KismetMathLibrary.FClamp` (.x (+ (`self.Pos`) (* _output_get (`self.LargoPaso`)))) _returnvalue_3 (- (* (.x (`self.Tamano`)) 0.5) 500.0)) (`KismetMathLibrary.FClamp` (.y (+ (`self.Pos`) (* _output_get (`self.LargoPaso`)))) (- 500.0 _returnvalue) (- _returnvalue 500.0)) (`KismetMathLibrary.FClamp` (.z (+ (`self.Pos`) (* _output_get (`self.LargoPaso`)))) (- 500.0 _returnvalue_2) (- _returnvalue_2 350.0)))))
    (`GeometryScriptLibrary_MeshPrimitiveFunctions.AppendSphereBox` (`self.MallaHerramienta`) (struct) (`KismetMathLibrary.MakeTransform` _output_get_2) (`KismetMathLibrary.RandomFloatInRangeFromStream` (`self.Stream`) (`self.RadioMin`) (`self.RadioMax`)) 5 5 5)
    (`KismetArrayLibrary.Array_Add` (`self.PuntosTunel`) (`KismetMathLibrary.TransformLocation` (`self.GetTransform`) _output_get_2)))
  (bind _returnvalue_7 (`BaseDynamicMeshComponent.GetDynamicMesh` (`self.GetDynamicMeshComponent`)))
  (`GeometryScriptLibrary_MeshBooleanFunctions.ApplyMeshSelfUnion` _mallaherramienta)
  (bind _returnvalue_8 (`GeometryScriptLibrary_MeshBooleanFunctions.ApplyMeshBoolean` _returnvalue_7 (struct) _mallaherramienta (struct) "Subtract"))
  (`GeometryScriptLibrary_MeshNormalsFunctions.ComputeSplitNormals` _returnvalue_8)
  (`self.ReleaseComputeMesh` (`self.MallaHerramienta`))
  (`DynamicMeshComponent.SetComplexAsSimpleCollisionEnabled` (`self.GetDynamicMeshComponent`) true true)
  (`KismetSystemLibrary.Delay` 1.5)
  (for _array_element (`self.PuntosTunel`)
    (if (`KismetMathLibrary.RandomBoolWithWeightFromStream` _stream (`self.ProbVeta`))
      (bind (_outhit _returnvalue_9) (`KismetSystemLibrary.LineTraceSingle` :`Start` _array_element :`End` (+ _array_element (* (`KismetMathLibrary.RandomUnitVectorFromStream` _stream) (1500.0 1500.0 1500.0))) :`TraceChannel` "TraceTypeQuery1" :`bTraceComplex` true :`bIgnoreSelf` false))
      (if _returnvalue_9
        (bind (_bblockinghit _binitialoverlap _time _distance _location _impactpoint _normal _impactnormal) (`GameplayStatics.BreakHitResult` _outhit))
        (bind _returnvalue_10 (`KismetMathLibrary.MakeRotFromX` _impactnormal))
        (`|SpawnActorFromClass` (`KismetArrayLibrary.Array_Get` _clasesveta (`KismetMathLibrary.RandomIntegerInRangeFromStream` _stream 0 (- (`KismetArrayLibrary.Array_Length` _clasesveta) 1))) (`KismetMathLibrary.MakeTransform` _impactpoint _returnvalue_10) "AlwaysSpawn" "MultiplyWithRoot" null null)
        (if (and (`KismetMathLibrary.RandomBoolWithWeightFromStream` _stream (`self.ProbAmbar`)) (< (.z _impactpoint) (.z (`self.K2_GetActorLocation`))))
          (`|SpawnActorFromClass` "/Game/Excavacion/BP_AmbarDino.BP_AmbarDino_C" (`KismetMathLibrary.MakeTransform` (- _impactpoint (* _impactnormal (260.0 260.0 260.0))) _returnvalue_10) "AlwaysSpawn" "MultiplyWithRoot" null null))))))

(event `Excavar`
  (bind _returnvalue (`self.AllocateComputeMesh`))
  (bind _output_get (set `self.MallaHerramienta` _returnvalue))
  (bind _returnvalue_2 (`GeometryScriptLibrary_MeshPrimitiveFunctions.AppendSphereBox` _output_get (struct) (`KismetMathLibrary.MakeTransform` (`KismetMathLibrary.InverseTransformLocation` (`self.GetTransform`) (`self.PuntoExcavar`))) (`self.RadioExcavar`) 3 3 3))
  (`GeometryScriptLibrary_MeshDeformFunctions.ApplyPerlinNoiseToMesh2` _returnvalue_2)
  (bind _returnvalue_3 (`BaseDynamicMeshComponent.GetDynamicMesh` (`self.GetDynamicMeshComponent`)))
  (bind _returnvalue_4 (`GeometryScriptLibrary_MeshBooleanFunctions.ApplyMeshBoolean` _returnvalue_3 (struct) (`self.MallaHerramienta`) (struct) "Subtract"))
  (`GeometryScriptLibrary_MeshNormalsFunctions.ComputeSplitNormals` _returnvalue_4)
  (`self.ReleaseComputeMesh` (`self.MallaHerramienta`))
  (`DynamicMeshComponent.SetComplexAsSimpleCollisionEnabled` (`self.GetDynamicMeshComponent`) true true))

(fn `UserConstructionScript`)