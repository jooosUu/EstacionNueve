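; BP_Veta is a mineable ore vein actor that gives the player a resource when hit.
; On BeginPlay it applies its vein material to the rock mesh and sets the glow light's color and intensity from variables.
; Any damage taken while the player is within range spends one hit and adds the configured resource to BP_Cyrus.
; The vein destroys itself once its hits run out.
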(event `self.ReceiveBeginPlay`
  (bind _brillo (`self.Brillo`))
  (`PrimitiveComponent.SetMaterial` (`self.Roca`) 0 (`self.MaterialVeta`))
  (`LightComponent.SetLightColor` _brillo (`self.ColorBrillo`) true)
  (`LightComponent.SetIntensity` _brillo (`self.IntensidadBrillo`)))

(event `self.ReceiveAnyDamage`
  (params (Damage :type "Float (single-precision)") (DamageType :type "DamageType Object Reference") (InstigatedBy :type "Controller Object Reference") (DamageCauser :type "Actor Object Reference"))
  (bind _returnvalue (`GameplayStatics.GetPlayerCharacter` 0))
  (if (<= (`self.GetDistanceTo` _returnvalue) 400.0)
    (bind _output_get (set `self.Golpes` (- (`self.Golpes`) 1)))
    (bind _asbp_cyrus (cast `/Game/Blueprints/BP_Cyrus` _returnvalue))
    (`/Game/Blueprints/BP_Cyrus.AgregarRecurso` _asbp_cyrus (`self.Recurso`) (`self.Cantidad`))
    (if (<= _output_get 0)
      (`self.K2_DestroyActor`))))

(fn `UserConstructionScript`)