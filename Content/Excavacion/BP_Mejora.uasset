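; BP_Mejora is a one-time upgrade station in the excavation game, with its title and cost shown on a text label.
; Pressing E nearby, polled on Tick, or calling Interactuar attempts the purchase using BP_Cyrus's money and an inventory resource.
; Success marks it bought, then Tipo selects the effect: wider dig radius on all BP_TerrenoExcavable actors, stronger player lamp, or revealing its structure.
; Insufficient funds or resources print the cost.
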(event `self.ReceiveTick`
  (params (DeltaSeconds :type "Float (single-precision)"))
  (bind _returnvalue (`GameplayStatics.GetPlayerCharacter` 0))
  (bind _titulo (`self.Titulo`))
  (bind _costoplata (`self.CostoPlata`))
  (bind _recursocosto (`self.RecursoCosto`))
  (bind _cantidadrecurso (`self.CantidadRecurso`))
  (bind _tipo (`self.Tipo`))
  (if (and (<= (`self.GetDistanceTo` _returnvalue) 320.0) (`PlayerController.WasInputKeyJustPressed` (`GameplayStatics.GetPlayerController` 0) "E"))
    (if (not (`self.Comprada`)) :!label _label
      (bind _asbp_cyrus (cast `/Game/Blueprints/BP_Cyrus` _returnvalue))
      (bind _money (`/Game/Blueprints/BP_Cyrus.Money` _asbp_cyrus))
      (bind _inventario (`/Game/Blueprints/BP_Cyrus.Inventario` _asbp_cyrus))
      (bind _value (`BlueprintMapLibrary.Map_Find` _inventario _recursocosto))
      (if (and (>= _money _costoplata) (>= _value _cantidadrecurso))
        (set `/Game/Blueprints/BP_Cyrus.Money` (- _money _costoplata) _asbp_cyrus)
        (`BlueprintMapLibrary.Map_Add` _inventario _recursocosto (- _value _cantidadrecurso))
        (set `self.Comprada` true)
        (`TextRenderComponent.K2_SetText` (`self.Texto`) (`KismetTextLibrary.Conv_StringToText` (`KismetStringLibrary.Concat_StrStr` "LISTO: " _titulo)))
        (`KismetSystemLibrary.PrintString` (`KismetStringLibrary.Concat_StrStr` "Mejora comprada: " _titulo) true true (struct :`R` 0.4 :`G` 1.0 :`B` 0.4 :`A` 1.0) 4.0)
        (if (== _tipo 0)
          (bind _outactors (`GameplayStatics.GetAllActorsOfClass` "/Game/Excavacion/BP_TerrenoExcavable.BP_TerrenoExcavable_C"))
          (for _array_element _outactors
            (set `/Game/Excavacion/BP_TerrenoExcavable.RadioExcavar` 210.0 _array_element))
          (elif (== _tipo 1)
            (bind _lampara (`/Game/Blueprints/BP_Cyrus.Lampara` _asbp_cyrus))
            (`LightComponent.SetIntensity` _lampara 16000.0)
            (`LocalLightComponent.SetAttenuationRadius` _lampara 2800.0)
            (elif (== _tipo 2)
              (`SceneComponent.SetVisibility` (`self.Estructura`) true true))))
        (else
          (`KismetSystemLibrary.PrintString` (`KismetStringLibrary.Concat_StrStr` (`KismetStringLibrary.Concat_StrStr` (`KismetStringLibrary.Concat_StrStr` (`KismetStringLibrary.Concat_StrStr` (`KismetStringLibrary.Concat_StrStr` "Te falta: $" (`KismetStringLibrary.Conv_IntToString` _costoplata)) " y ") (`KismetStringLibrary.Conv_IntToString` _cantidadrecurso)) " ") (`KismetStringLibrary.Conv_NameToString` _recursocosto)) true true (struct :`R` 1.0 :`G` 0.4 :`B` 0.3 :`A` 1.0)))))))

(event `self.ReceiveBeginPlay`
  (`TextRenderComponent.K2_SetText` (`self.Texto`) (`KismetTextLibrary.Conv_StringToText` (`KismetStringLibrary.Concat_StrStr` (`KismetStringLibrary.Concat_StrStr` (`KismetStringLibrary.Concat_StrStr` (`KismetStringLibrary.Concat_StrStr` (`KismetStringLibrary.Concat_StrStr` (`KismetStringLibrary.Concat_StrStr` (`self.Titulo`) "\n[E] $") (`KismetStringLibrary.Conv_IntToString` (`self.CostoPlata`))) " + ") (`KismetStringLibrary.Conv_IntToString` (`self.CantidadRecurso`))) " ") (`KismetStringLibrary.Conv_NameToString` (`self.RecursoCosto`))))))

(event `Interactuar`
  (goto _label))

(fn `UserConstructionScript`)