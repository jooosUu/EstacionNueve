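; BP_AmbarDino is a harvestable excavation node that yields amber and fossils.
; On any damage, if player 0's character is within range, it loses a hit point from Golpes and grants amber to BP_Cyrus through AgregarRecurso.
; When Golpes runs out it also awards a fossil and destroys itself.
; The range check measures the player character, not the damage causer, and the damage amount is ignored.
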(event `self.ReceiveAnyDamage`
  (params (Damage :type "Float (single-precision)") (DamageType :type "DamageType Object Reference") (InstigatedBy :type "Controller Object Reference") (DamageCauser :type "Actor Object Reference"))
  (bind _returnvalue (`GameplayStatics.GetPlayerCharacter` 0))
  (if (<= (`self.GetDistanceTo` _returnvalue) 450.0)
    (bind _output_get (set `self.Golpes` (- (`self.Golpes`) 1)))
    (bind _asbp_cyrus (cast `/Game/Blueprints/BP_Cyrus` _returnvalue))
    (`/Game/Blueprints/BP_Cyrus.AgregarRecurso` _asbp_cyrus "Ambar" 2)
    (if (<= _output_get 0)
      (`/Game/Blueprints/BP_Cyrus.AgregarRecurso` _asbp_cyrus "Fosil" 1)
      (`self.K2_DestroyActor`))))

(fn `UserConstructionScript`)