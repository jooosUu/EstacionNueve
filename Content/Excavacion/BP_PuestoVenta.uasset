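; BP_PuestoVenta is a sales stand where the player character, BP_Cyrus, sells inventory items for money.
; A sale runs from the Interactuar event, or from Tick polling for the E key while the player is within range.
; It loops over the keys of the Precios map, totals quantity times price, and removes those entries from Inventario.
; The total is added to Cyrus's Money and printed on screen.
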(event `self.ReceiveTick`
  (params (DeltaSeconds :type "Float (single-precision)"))
  (bind _returnvalue (`GameplayStatics.GetPlayerCharacter` 0))
  (bind _precios (`self.Precios`))
  (bind _total (`self.Total`))
  (if (and (<= (`self.GetDistanceTo` _returnvalue) 320.0) (`PlayerController.WasInputKeyJustPressed` (`GameplayStatics.GetPlayerController` 0) "E"))
    (bind _asbp_cyrus (cast `/Game/Blueprints/BP_Cyrus` _returnvalue :!label _label))
    (set `self.Total` 0)
    (bind _keys (`BlueprintMapLibrary.Map_Keys` _precios))
    (for _array_element _keys
      (bind _inventario (`/Game/Blueprints/BP_Cyrus.Inventario` _asbp_cyrus))
      (set `self.Total` (+ (`self.Total`) (* (`BlueprintMapLibrary.Map_Find` _inventario _array_element) (`BlueprintMapLibrary.Map_Find` _precios _array_element))))
      (`BlueprintMapLibrary.Map_Remove` _inventario _array_element))
    (set `/Game/Blueprints/BP_Cyrus.Money` (+ (`/Game/Blueprints/BP_Cyrus.Money` _asbp_cyrus) _total) _asbp_cyrus)
    (`KismetSystemLibrary.PrintString` (`KismetStringLibrary.Concat_StrStr` "Vendiste todo por $" (`KismetStringLibrary.Conv_IntToString` _total)) true true (struct :`R` 0.4 :`G` 1.0 :`B` 0.4 :`A` 1.0) 3.0)))

(event `Interactuar`
  (goto _label))

(fn `UserConstructionScript`)