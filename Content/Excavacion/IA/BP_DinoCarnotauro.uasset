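; Carnotaurus dinosaur Blueprint for the excavation area, with simple logic to chase the player.
; On Tick it checks the distance to player 0, then smoothly turns on yaw toward them with RInterpTo and moves forward through AddMovementInput.
; The distance threshold is zero, so the chase branch never runs as written.
; BeginPlay, overlap and the construction script are empty.
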(event `self.ReceiveTick`
  (params (DeltaSeconds :type "Float (single-precision)"))
  (bind _returnvalue (`GameplayStatics.GetPlayerCharacter` 0))
  (if (< (`self.GetDistanceTo` _returnvalue) 0.0)
    (`self.K2_SetActorRotation` (`KismetMathLibrary.RInterpTo` (`self.K2_GetActorRotation`) (`KismetMathLibrary.MakeRotator` 0.0 0.0 (.yaw (`KismetMathLibrary.FindLookAtRotation` (`self.K2_GetActorLocation`) (`self.K2_GetActorLocation` _returnvalue)))) DeltaSeconds))
    (`self.AddMovementInput` (`self.GetActorForwardVector`))))

(fn `UserConstructionScript`)