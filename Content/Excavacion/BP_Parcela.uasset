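; BP_Parcela is a farm plot where the player plants a fern, waits for it to grow and harvests Forraje.
; A three-state Estado switches the plant's visibility and the prompt text, and harvesting adds the resource to BP_Cyrus through a cast.
; Tick handles both proximity-checked E-key polling and timed growth, lerping the plant's scale until ready.
; An Interactuar event jumps into the same sow-or-harvest logic.
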(event `self.ReceiveTick`
  (params (DeltaSeconds :type "Float (single-precision)"))
  (bind _returnvalue (`GameplayStatics.GetPlayerCharacter` 0))
  (bind _estado (`self.Estado`))
  (bind _texto (`self.Texto`))
  (bind _planta (`self.Planta`))
  (`|ExecutionSequence`
    (:`then_0`
      (if (and (<= (`self.GetDistanceTo` _returnvalue) 320.0) (`PlayerController.WasInputKeyJustPressed` (`GameplayStatics.GetPlayerController` 0) "E"))
        (if (== _estado 0) :!label _label
          (set `self.Estado` 1)
          (set `self.Progreso` 0.0)
          (`SceneComponent.SetVisibility` _planta true false)
          (`TextRenderComponent.K2_SetText` _texto (`KismetTextLibrary.Conv_StringToText` "Creciendo..."))
          (elif (== _estado 2)
            (bind _asbp_cyrus (cast `/Game/Blueprints/BP_Cyrus` _returnvalue))
            (`/Game/Blueprints/BP_Cyrus.AgregarRecurso` _asbp_cyrus "Forraje" 3)
            (set `self.Estado` 0)
            (`SceneComponent.SetVisibility` _planta false false)
            (`TextRenderComponent.K2_SetText` _texto (`KismetTextLibrary.Conv_StringToText` "PARCELA\n[E] Sembrar helecho"))))))
    (:`then_1`
      (if (== _estado 1)
        (bind _output_get (set `self.Progreso` (+ (`self.Progreso`) (/ DeltaSeconds (`self.TiempoCrecer`)))))
        (bind _returnvalue_2 (`KismetMathLibrary.Lerp` 0.05 0.6 _output_get))
        (`SceneComponent.SetRelativeScale3D` _planta (`KismetMathLibrary.MakeVector` _returnvalue_2 _returnvalue_2 (`KismetMathLibrary.Lerp` 0.4 2.5 _output_get)))
        (if (>= _output_get 1.0)
          (set `self.Estado` 2)
          (`TextRenderComponent.K2_SetText` _texto (`KismetTextLibrary.Conv_StringToText` "LISTO\n[E] Cosechar")))))))

(event `Interactuar`
  (goto _label))

(fn `UserConstructionScript`)